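; Pawn movement component that drives its owner's physics-simulated box root from movement input.
; Tick consumes and normalizes the pawn's input vector, while a looping timer runs a fixed 250 Hz step.
; Each step applies acceleration with planar drag unless sphere or box traces find blockers ahead, then writes the velocity back to the box.
; Engine gravity handles falling; the custom gravity function is called disabled.
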(event `self.ReceiveBeginPlay`
  (bind _aspawn (cast `Pawn` (`self.GetOwner`)))
  (bind _output_get (set `self.parent_pawn` _aspawn))
  (bind _asbox_collision (cast `BoxComponent` (`Actor.RootComponent` _output_get)))
  (set `self.collision_box` _asbox_collision)
  (`self.configure_physics`)
  (bind _output_get_2 (set `self.delta_time` (/ 1.0 250.0)))
  (`KismetSystemLibrary.K2_SetTimerDelegate` (delegate `Fixed_tick`) _output_get_2 true))

(event `self.ReceiveTick`
  (params (DeltaSeconds :type "Float (single-precision)"))
  (bind _parent_pawn (`self.parent_pawn`)
    (:`then`
      (bind _returnvalue (`Pawn.ConsumeMovementInputVector` _parent_pawn))
      (set `self.input` (`KismetMathLibrary.Normal` _returnvalue)))
    (:`else`)))

(event `Fixed_tick`
  (bind _returnvalue (`SceneComponent.K2_GetComponentLocation` (`self.collision_box`)))
  (bind _returnvalue_2 (`SceneComponent.K2_GetComponentLocation` (`self.collision_box`)))
  (set `self.velocity` (`SceneComponent.GetComponentVelocity` (`self.collision_box`)))
  (`self.apply_gravity` false)
  (bind (_outhit _returnvalue_3) (`KismetSystemLibrary.SphereTraceSingleForObjects` :`Start` _returnvalue_2 :`End` (+ (* (`self.input`) (`self.trace_range`)) _returnvalue_2) :`Radius` (`self.Trace_raious`) :`ObjectTypes` (`|MakeArray` "ObjectTypeQuery1" "ObjectTypeQuery10" :!type "EObjectTypeQuery Enum") :`DrawDebugType` "ForOneFrame"))
  (if (not _returnvalue_3)
    (bind (_outhit_2 _returnvalue_4) (`KismetSystemLibrary.BoxTraceSingleForObjects` :`Start` _returnvalue :`End` (+ (* (`self.input`) 70.0) _returnvalue) :`HalfSize` (`BoxComponent.BoxExtent` (`self.collision_box`)) :`ObjectTypes` (`|MakeArray` "ObjectTypeQuery3" :!type "EObjectTypeQuery Enum") :`DrawDebugType` "ForOneFrame"))
    (if (not _returnvalue_4)
      (`self.Movement_velocity` (`self.max_speed`) (`self.Acceleration`))))
  (`PrimitiveComponent.SetAllPhysicsLinearVelocity` (`self.collision_box`) (`self.velocity`) false))

(fn `apply_gravity`
  (params (appl_gravity :type Boolean))
  (if appl_gravity
    (set `self.velocity` (+ (`self.velocity`) (* (* (`self.Gravity_direction`) (`KismetSystemLibrary.MakeLiteralDouble` (`self.gravity`))) (`self.delta_time`))))))

(fn `configure_physics`
  (`self.SetTickGroup` "TG_PostPhysics")
  (`PrimitiveComponent.SetSimulatePhysics` (`self.collision_box`) true)
  (`PrimitiveComponent.SetEnableGravity` (`self.collision_box`) true)
  (`PrimitiveComponent.SetPhysMaterialOverride` (`self.collision_box`) (`self.physical_material`)))

(fn `Movement_velocity`
  (params (Max_speed :type "Float (double-precision)") (Acceleration :type "Float (double-precision)"))
  (set `self.velocity` (+ (* (- (* (* (`self.input`) Max_speed) Acceleration) (* (`KismetMathLibrary.ProjectVectorOnToPlane` (`self.velocity`) (`self.Gravity_direction`)) Acceleration)) (`self.delta_time`)) (`self.velocity`))))
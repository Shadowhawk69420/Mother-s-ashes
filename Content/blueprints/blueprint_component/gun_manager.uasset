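; Gun manager component for Player_character that runs one weapon's equip, idle, shoot, reload, fall and land behavior.
; Timers sequence the states through ready, reload and reloading flags, with deactivation clearing all timers.
; Each state plays first-person arm animations, passing them to the owner for third person, with empty-gun variants.
; Shots sphere-trace from the camera, send random damage via interface, update the color-lerped ammo text and auto-reload when empty.
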(event `land`
  (bind _arms_land (`self.arms_land`))
  ;[1 1 1] land
  (`SkeletalMeshComponent.PlayAnimation` (`self.FP_Arms`) _arms_land false)
  (`self.set_tp_anim` _arms_land)
  (bind _returnvalue (`KismetSystemLibrary.K2_SetTimerDelegate` (delegate `land_reset`) (`self.land_recover_delay`)))
  (set `self.Land_recover_timer` _returnvalue)
  (`KismetSystemLibrary.K2_ClearAndInvalidateTimerHandle` (`self.Fall_idle_timer`)))

(event `land_reset`
  ;[1 1 1] land
  (`self.idle` true))

(event `Fall_or_jump`
  (bind _arms_fall (`self.arms_fall`))
  ;[1 1 1] fall_or_jump
  (`/Engine/EditorBlueprintResources/StandardMacros.DoOnce` false :!label _label
    (:`Completed`
      (`self.deactivate_weapon`)
      (`SkeletalMeshComponent.PlayAnimation` (`self.FP_Arms`) _arms_fall false)
      (`self.set_tp_anim` _arms_fall)
      (`SkeletalMeshComponent.PlayAnimation` (`self.gun_mesh`) (select `bool` (>= (`self.bullets`) 1.0) :`false` (`self.gun_idle_empty`) :`true` (`self.gun_idle`) :!type "AnimationAsset Object Reference") false)
      (bind _returnvalue (`KismetSystemLibrary.K2_SetTimerDelegate` (delegate `fall_idle_anim`) (`self.fall_delay`)))
      (set `self.Fall_idle_timer` _returnvalue))))

(event `reset_fall`
  ;[1 1 1] fall_or_jump
  (goto _label :!via `Reset`))

(event `fall_idle_anim`
  (bind _arms_fall_idle (`self.arms_fall_idle`))
  ;[1 1 1] fall_or_jump
  (`SkeletalMeshComponent.PlayAnimation` (`self.FP_Arms`) _arms_fall_idle true)
  (`self.set_tp_anim` _arms_fall_idle))

(event `self.ReceiveBeginPlay`
  (bind _asplayer_character (cast `/Game/blueprints/player_characters/Player_character` (`self.GetOwner`)))
  (bind _output_get (set `self.owner` _asplayer_character))
  (set `self.FP_Arms` (`/Game/blueprints/player_characters/Player_character.fp_arms` _output_get))
  (set `self.gun_mesh` (`/Game/blueprints/player_characters/Player_character.gun_mesh` _output_get))
  (set `self.fp_camera` (`/Game/blueprints/player_characters/Player_character.fp_cam` _output_get))
  (set `self.text_info` (`/Game/blueprints/player_characters/Player_character.weapon_ammo_counter` _asplayer_character)))

(event `Activate_weapon`
  (bind _arm_equip (`self.arm_equip`))
  ;[1 1 1] equiping and idle
  (`SkeletalMeshComponent.PlayAnimation` (`self.FP_Arms`) _arm_equip false)
  (`self.set_tp_anim` _arm_equip)
  (`self.Set_weapon_idle_empty_or_not_anim`)
  (`self.update_text`)
  (bind _returnvalue (`KismetSystemLibrary.K2_SetTimerDelegate` (delegate `to_idle`) (`self.equip_anim_delay`)))
  (set `self.Timers_equip` _returnvalue))

(event `Set_weapon_idle_empty_or_not_anim`
  ;[1 1 1] equiping and idle
  (`SkeletalMeshComponent.PlayAnimation` (`self.gun_mesh`) (select `bool` (>= (`self.bullets`) 1.0) :`false` (`self.gun_idle_empty`) :`true` (`self.gun_idle`) :!type "AnimationAsset Object Reference") true))

(event `to_idle`
  ;[1 1 1] equiping and idle
  (`self.idle` true)
  (`self.check_ammo_none`
    (:`no_ammo`
      (set `self.can_reload` true)
      (`self.reload_gun`))))

(event `reload_gun`
  (bind _arm_reload_empty (`self.arm_reload_empty`))
  (bind _arm_reload (`self.arm_reload`))
  ;[1 1 1] RELOAD
  (if (`self.can_reload`)
    (`KismetSystemLibrary.K2_ClearAndInvalidateTimerHandle` (`self.from_shoot_anim_to_idle_timer`))
    (set `self.can_reload` false)
    (set `self.reloading` true)
    (if (< (`self.bullets`) (`self.bulletsmax`))
      (if (>= (`self.bullets`) 1.0)
        (`SkeletalMeshComponent.PlayAnimation` (`self.FP_Arms`) _arm_reload false)
        (`self.set_tp_anim` _arm_reload)
        (`SkeletalMeshComponent.PlayAnimation` (`self.gun_mesh`) (`self.gun_reload`) false)
        (bind _returnvalue (`KismetSystemLibrary.K2_SetTimerDelegate` (delegate `give_ammo`) (`self.Reload_delay`)))
        (set `self.reload_timer_1+round` _returnvalue)
        (else
          (`SkeletalMeshComponent.PlayAnimation` (`self.FP_Arms`) _arm_reload_empty false)
          (`self.set_tp_anim` _arm_reload_empty)
          (`SkeletalMeshComponent.PlayAnimation` (`self.gun_mesh`) (`self.gun_reload_empty`) false)
          (bind _returnvalue_2 (`KismetSystemLibrary.K2_SetTimerDelegate` (delegate `give_ammo`) (`self.Reload_delay_empty`)))
          (set `self.reload_timer_empty` _returnvalue_2))))))

(event `idle`
  (params (play_anim :type Boolean :default true))
  (bind _arm_idle (`self.arm_idle`))
  ;[1 1 1] equiping and idle
  (if play_anim
    (`SkeletalMeshComponent.PlayAnimation` (`self.FP_Arms`) _arm_idle true)
    (`self.set_tp_anim` _arm_idle)
    (`self.Set_weapon_idle_empty_or_not_anim`))
  (`self.reset_fall`)
  (set `self.ready_to_fire` true)
  (set `self.can_reload` true)
  (set `self.reloading` false))

(event `give_ammo`
  ;[1 1 1] RELOAD
  (set `self.bullets` (`self.bulletsmax`))
  (`self.update_text`)
  (`self.idle` true)
  (set `self.reloading` false))

(event `deactivate_weapon`
  ;[1 1 1] reseting stuff
  (`KismetSystemLibrary.K2_ClearAndInvalidateTimerHandle` (`self.Timers_equip`))
  (`KismetSystemLibrary.K2_ClearAndInvalidateTimerHandle` (`self.shot_timer`))
  (`KismetSystemLibrary.K2_ClearAndInvalidateTimerHandle` (`self.reload_timer_1+round`))
  (`KismetSystemLibrary.K2_ClearAndInvalidateTimerHandle` (`self.reload_timer_empty`))
  (`KismetSystemLibrary.K2_ClearAndInvalidateTimerHandle` (`self.Land_recover_timer`))
  (`KismetSystemLibrary.K2_ClearAndInvalidateTimerHandle` (`self.Fall_idle_timer`))
  (`KismetSystemLibrary.K2_ClearAndInvalidateTimerHandle` (`self.from_shoot_anim_to_idle_timer`))
  (set `self.ready_to_fire` false)
  (set `self.can_reload` false)
  (set `self.reloading` false))

(event `shoot`
  (bind _arm_shoot (`self.arm_shoot`))
  (bind _returnvalue (`SceneComponent.K2_GetComponentLocation` (`self.fp_camera`)))
  ;[1 1 1] weapon_shooting
  (if (`self.ready_to_fire`)
    (if (>= (`self.bullets`) 1.0)
      (if (not (`self.reloading`))
        (set `self.ready_to_fire` false)
        (set `self.can_reload` false)
        (set `self.bullets` (- (`self.bullets`) 1.0))
        (`SkeletalMeshComponent.PlayAnimation` (`self.FP_Arms`) _arm_shoot false)
        (`self.set_tp_anim` _arm_shoot)
        (`KismetSystemLibrary.K2_ClearAndInvalidateTimerHandle` (`self.from_shoot_anim_to_idle_timer`))
        (bind _returnvalue_2 (`KismetSystemLibrary.K2_SetTimerDelegate` (delegate `back_to_idle`) (`self.from_shoot_to_idle`)))
        (set `self.from_shoot_anim_to_idle_timer` _returnvalue_2)
        (`SkeletalMeshComponent.PlayAnimation` (`self.gun_mesh`) (select `bool` (>= (`self.bullets`) 1.0) :`false` (`self.gun_shoot_empty`) :`true` (`self.gun_shoot`) :!type "AnimationAsset Object Reference") false)
        (bind _outhit (`KismetSystemLibrary.SphereTraceSingleForObjects` :`Start` _returnvalue :`End` (+ _returnvalue (* (`SceneComponent.GetForwardVector` (`self.fp_camera`)) 2500.0)) :`Radius` 7.0 :`ObjectTypes` (`|MakeArray` "ObjectTypeQuery1" "ObjectTypeQuery2" "ObjectTypeQuery3" :!type "EObjectTypeQuery Enum") :`DrawDebugType` "ForOneFrame"))
        (`GameplayStatics.PlayWorldCameraShake` "/Game/blueprints/camera_shakes/Shoot_shake.Shoot_shake_C" (`SceneComponent.K2_GetComponentLocation` (`self.fp_camera`)) 20.0 20.0 1.0 true)
        (`|ExecutionSequence`
          (:`then_0`
            (`self.update_text`)
            (bind (_bblockinghit _binitialoverlap _time _distance _location _impactpoint _normal _impactnormal _physmat _hitactor) (`GameplayStatics.BreakHitResult` _outhit))
            (if (`KismetSystemLibrary.DoesImplementInterface` _hitactor "/Game/blueprints/interfaces/Damage.Damage_C")
              (message `/Game/blueprints/interfaces/Damage.Normal_damage` _hitactor (`KismetMathLibrary.RandomIntegerInRange` (`self.damage_min`) (`self.damage_max`)))))
          (:`then_1`
            (bind _returnvalue_3 (`KismetSystemLibrary.K2_SetTimerDelegate` (delegate `Shot_reset`) (`self.Trigger_relese_delay`)))
            (set `self.shot_timer` _returnvalue_3)))))))

(event `back_to_idle`
  ;[1 1 1] weapon_shooting
  (`self.idle` true))

(event `Shot_reset`
  ;[1 1 1] weapon_shooting
  (`self.idle` false)
  (`self.check_ammo_none`
    (:`no_ammo`
      (set `self.can_reload` true)
      (`self.reload_gun`))))

(fn `set_tp_anim`
  (params (Gun_animation :type "AnimSequenceBase Object Reference"))
  (set `/Game/blueprints/player_characters/Player_character.Gun_animation` Gun_animation (`self.owner`)))

(fn `update_text`
  (`TextRenderComponent.K2_SetText` (`self.text_info`) (`|FormatText` "[{Bullets}]" (`KismetMathLibrary.FTrunc` (`self.bullets`))))
  (`TextRenderComponent.SetTextRenderColor` (`self.text_info`) (`KismetMathLibrary.Conv_LinearColorToColor` (`KismetMathLibrary.LinearColorLerp` (struct :`R` 1.0 :`A` 1.0) (struct :`G` 1.0 :`A` 1.0) (/ (`self.bullets`) (`self.bulletsmax`))))))
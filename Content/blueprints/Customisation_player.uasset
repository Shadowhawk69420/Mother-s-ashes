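; Player customisation Blueprint that applies saved colours to the explorer mask and personal light tool.
; BeginPlay creates dynamic material instances for the light glow, mask and lens before calling the parent BeginPlay.
; UpdateCustomisation calls the parent, loads the "customisation" save slot, then sets material colour parameters.
; The saved flashlight colour drives both light and lens and is stored as LightColor, while the primary colour feeds the mask's tertiary channel.
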(event `self.Update_customisation`
  (`parent.Update_customisation`)
  (bind _returnvalue (`GameplayStatics.LoadGameFromSlot` "customisation"))
  (bind _ascustomisation (cast `/Game/Customisation` _returnvalue))
  (bind _output_get (set `self.light_color` (`/Game/Customisation.Flashlight_color` _ascustomisation)))
  (`MaterialInstanceDynamic.SetVectorParameterValue` (`self.Personal_light`) "color" _output_get)
  (`MaterialInstanceDynamic.SetVectorParameterValue` (`self.Mask+mat`) "Tetiary_color" (`/Game/Customisation.Primary_color` _ascustomisation))
  (`MaterialInstanceDynamic.SetVectorParameterValue` (`self.Mask_lens_mat`) "Primary_color" (`/Game/Customisation.Flashlight_color` _ascustomisation)))

(event `self.ReceiveBeginPlay`
  (bind _returnvalue (`PrimitiveComponent.CreateDynamicMaterialInstance` (`self.personal_light_tool`) 1 "/Game/Materials/personal_light_glow.personal_light_glow" "None"))
  (set `self.Personal_light` _returnvalue)
  (bind _returnvalue_2 (`PrimitiveComponent.CreateDynamicMaterialInstance` (`self.Mask`) 0 "/Game/Materials/Explorer_mask.Explorer_mask" "None"))
  (set `self.Mask+mat` _returnvalue_2)
  (bind _returnvalue_3 (`PrimitiveComponent.CreateDynamicMaterialInstance` (`self.Mask`) 1 "/Game/Materials/Mask_lens_Inst.Mask_lens_Inst" "None"))
  (set `self.Mask_lens_mat` _returnvalue_3)
  (`parent.ReceiveBeginPlay`))

(fn `UserConstructionScript`
  (`parent.UserConstructionScript`))
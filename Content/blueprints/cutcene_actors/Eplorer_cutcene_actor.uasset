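; Cutscene actor for the Explorer character that can show the player's saved colour customisation and a powers glow.
; When customisation is enabled, BeginPlay creates dynamic materials for body, face, hair and gear, then applies colours from the "customisation" save slot, creating it if missing.
; Body and face glow in the flashlight colour with powers, otherwise black.
; Tick waits for HasPowers, refreshes the look once, then disables itself.
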(event `self.ReceiveTick`
  (params (DeltaSeconds :type "Float (single-precision)"))
  (if (`self.Has_powers`)
    (`/Engine/EditorBlueprintResources/StandardMacros.DoOnce` false
      (:`Completed`
        (`self.Check_for_powar`)
        (`self.Update_customisation`)
        (`self.SetActorTickEnabled` false)))))

(event `Check_for_powar`
  (set `self.Has_powers` true)
  (`MaterialInstanceDynamic.SetVectorParameterValue` (`self.Explorer_body`) "Glow_color" (`self.flashlight_color`) :!label _label)
  (`MaterialInstanceDynamic.SetVectorParameterValue` (`self.explorer_face`) "Glow_color" (`self.flashlight_color`)))

(event `Update_customisation`
  (bind _returnvalue (`GameplayStatics.DoesSaveGameExist` "customisation"))
  (if (not _returnvalue)
    (bind _returnvalue_2 (`GameplayStatics.CreateSaveGameObject` "/Game/Customisation.Customisation_C"))
    (`GameplayStatics.SaveGameToSlot` _returnvalue_2 "customisation"))
  (bind _returnvalue_3 (`GameplayStatics.LoadGameFromSlot` "customisation"))
  (bind _ascustomisation (cast `/Game/Customisation` _returnvalue_3))
  (set `self.Primary_color` (`/Game/Customisation.Primary_color` _ascustomisation))
  (set `self.Secondary_color` (`/Game/Customisation.Shoe_color` _ascustomisation))
  (set `self.Hair_color` (`/Game/Customisation.Hair_color` _ascustomisation))
  (set `self.Top_color` (`/Game/Customisation.Top_color` _ascustomisation))
  (set `self.Backpack_color` (`/Game/Customisation.Backpack_color` _ascustomisation))
  (set `self.flashlight_color` (`/Game/Customisation.Flashlight_color` _ascustomisation))
  (`|ExecutionSequence`
    (:`then_0`
      (if (`self.Has_powers`)
        (goto _label)
        (else
          (`MaterialInstanceDynamic.SetVectorParameterValue` :`self` (`self.Explorer_body`) :`ParameterName` "Glow_color")
          (`MaterialInstanceDynamic.SetVectorParameterValue` :`self` (`self.explorer_face`) :`ParameterName` "Glow_color"))))
    (:`then_1`
      (`MaterialInstanceDynamic.SetVectorParameterValue` (`self.Explorer_body`) "Primary_color" (`self.Primary_color`))
      (`MaterialInstanceDynamic.SetVectorParameterValue` (`self.Explorer_gear`) "Primary_color" (`self.Primary_color`))
      (`MaterialInstanceDynamic.SetVectorParameterValue` (`self.Explorer_body`) "Secondary_color" (`self.Secondary_color`))
      (`MaterialInstanceDynamic.SetVectorParameterValue` (`self.Hair_material`) "Primary_color" (`self.Hair_color`))
      (`MaterialInstanceDynamic.SetVectorParameterValue` (`self.Explorer_body`) "Tetiary_color" (`self.Top_color`))
      (`MaterialInstanceDynamic.SetVectorParameterValue` (`self.Explorer_gear`) "Primary_color" (`self.Backpack_color`))
      (`MeshComponent.SetVectorParameterValueOnMaterials` (`self.SkeletalMeshComponent`) "color" (`KismetMathLibrary.Conv_LinearColorToVector` (`self.flashlight_color`))))))

(event `self.ReceiveBeginPlay`
  (if (`self.uses_customisation_options`)
    (bind _returnvalue (`PrimitiveComponent.CreateDynamicMaterialInstance` (`self.SkeletalMeshComponent`) 1 (`self.face_material_surce`) "None"))
    (set `self.explorer_face` _returnvalue)
    (bind _returnvalue_2 (`PrimitiveComponent.CreateDynamicMaterialInstance` (`self.SkeletalMeshComponent`) 0 (`self.explorer_body_surce`) "None"))
    (set `self.Explorer_body` _returnvalue_2)
    (bind _returnvalue_3 (`PrimitiveComponent.CreateDynamicMaterialInstance` (`self.SkeletalMeshComponent`) 2 "/Game/Materials/Explorer_hair.Explorer_hair" "None"))
    (set `self.Hair_material` _returnvalue_3)
    (bind _returnvalue_4 (`PrimitiveComponent.CreateDynamicMaterialInstance` (`self.SkeletalMeshComponent`) 6 "/Game/Materials/Explorer_gear.Explorer_gear" "None"))
    (set `self.Explorer_gear` _returnvalue_4)
    (`self.Update_customisation`)))

(fn `OnRep_Has_powers`)

(fn `UserConstructionScript`)
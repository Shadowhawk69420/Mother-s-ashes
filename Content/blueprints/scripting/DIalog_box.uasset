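; A scriptable dialog actor that plays a sequence of talker lines and optional player replies through the third-person HUD.
; A script message starts it after a delay, caching the player controller and HUD, and Switch_text_line advances through the Text array with brief input locking.
; A line can echo the reply chosen on the previous one.
; At the end it closes the box and sends script messages to either default actors or those tied to the final reply.
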(event `Switch_text_line`
  (params (chosen_reply :type Integer :default -1))
  (bind (_output_talker_name _output_talkertext _output_show_replies _output_reply_options) (break `/Game/blueprints/Blueprint_structures/Text_box_struct` (`|GetArrayItem` (`self.Text`) (`self.Current_box_index`))))
  (bind (_output_talker_name_2 _output_talkertext_2 _output_show_replies_2 _output_reply_options_2 _output_reply_of_actors_to_activate _output_usereplyastext) (break `/Game/blueprints/Blueprint_structures/Text_box_struct` (`|GetArrayItem` (`self.Text`) (`self.Current_box_index`))))
  (bind (_output_talker_name_3 _output_talkertext_3 _output_show_replies_3 _output_reply_options_3) (break `/Game/blueprints/Blueprint_structures/Text_box_struct` (`|GetArrayItem` (`self.Text`) (- (`self.Current_box_index`) 1))))
  (bind (_output_talker_name_4 _output_talkertext_4 _output_show_replies_4 _output_reply_options_4 _output_reply_of_actors_to_activate_2) (break `/Game/blueprints/Blueprint_structures/Text_box_struct` (`|GetArrayItem` (`self.Text`) (- (`self.Current_box_index`) 1))))
  (set `self.Chosen_reply` chosen_reply)
  (set `self.Can_press_enter` false)
  (set `self.Current_box_index` (+ (`self.Current_box_index`) 1))
  (if (>= (`self.Current_box_index`) (`KismetArrayLibrary.Array_Length` (`self.Text`))) :!label _label
    (set `self.Can_press_enter` false)
    (set `self.in_selection` false)
    (`/Game/blueprints/game_settings/Third_person_hud.Create_dialog_box` (`self.Third_person_hud`) "" "" false true false (`|MakeArray` "" :!type "Text"))
    (if (== (`self.Chosen_reply`) -1)
      (set `self.chosen_actors` (`self.actors_to_activate`))
      (else
        (set `self.chosen_actors` (`.actorstoactivate_3_6C7ACBB54F2B2905E5079AB0C1759BFE` (break `/Game/blueprints/Blueprint_structures/Actors_to_activate_array` (`|GetArrayItem` _output_reply_of_actors_to_activate_2 (`self.Chosen_reply`)))))))
    (for _array_element (`self.chosen_actors`)
      (message `/Game/blueprints/scripting/base/Scripting_events.Recive_script` _array_element (`GameplayStatics.GetPlayerCharacter` 0)))
    (set `self.activated` false)
    (else
      (if _output_usereplyastext
        (set `self.text_to_say` (`|GetArrayItem` _output_reply_options_3 (`self.Chosen_reply`)))
        (else
          (set `self.text_to_say` _output_talkertext)))
      (set `self.in_selection` _output_show_replies)
      (`/Game/blueprints/game_settings/Third_person_hud.Create_dialog_box` (`self.Third_person_hud`) (`KismetTextLibrary.Conv_StringToText` (`|GetEnumeratorNameAsString` _output_talker_name)) (`self.text_to_say`) true false _output_show_replies _output_reply_options)
      (`KismetSystemLibrary.Delay` 0.1)
      (set `self.Can_press_enter` true))))

(event `self.recive_script_multi`
  (params (Player_activator :type "Character Object Reference"))
  (set `self.Can_press_enter` false)
  (`KismetSystemLibrary.Delay` (`self.Start_delay`))
  (if (not (`self.activated`))
    (set `self.Current_box_index` 0)
    (bind _asthird_person_controller (cast `/Game/blueprints/game_settings/third_person_controller` (`Pawn.GetController` Player_activator)))
    (set `self.Player_controller` _asthird_person_controller)
    (bind _asthird_person_hud (cast `/Game/blueprints/game_settings/Third_person_hud` (`PlayerController.GetHUD` _asthird_person_controller)))
    (set `self.Third_person_hud` _asthird_person_hud)
    (set `self.activated` true)
    (goto _label)))

(fn `UserConstructionScript`
  (`parent.UserConstructionScript`))
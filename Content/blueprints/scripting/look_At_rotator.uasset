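; Scripting actor that smoothly turns a target actor, or player character 0 when the Player flag is set, to a preset orientation.
; The ReciveScript event waits a configurable delay, then captures the target's current rotation and plays a timeline.
; The timeline blends along the shortest path to this actor's root world rotation, so the placed orientation defines the result, with no look-at calculation despite the name.
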(event `/Game/blueprints/scripting/base/Scripting_events.Recive_script`
  (params (player_activator :type "Character Object Reference"))
  (`KismetSystemLibrary.Delay` (`self.Delay`))
  (if (`self.player`)
    (set `self.actor_to_rotate` (`GameplayStatics.GetPlayerCharacter` 0)))
  (set `self.actor_rotation` (`self.K2_GetActorRotation` (`self.actor_to_rotate`)))
  (bind (_direction _alpha) (`Timeline|Timeline_0` :`NewTime` 0.0 :!via `PlayFromStart`)
    (:`Update`
      (`self.K2_SetActorRotation` (`self.actor_to_rotate`) (`KismetMathLibrary.RLerp` (`self.actor_rotation`) (`SceneComponent.K2_GetComponentRotation` (`self.DefaultSceneRoot`)) _alpha true) true))))

(fn `UserConstructionScript`
  (`parent.UserConstructionScript`))
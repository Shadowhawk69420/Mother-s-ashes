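; Scripted trigger actor that transforms the Ghost_girl character into another form and glides her to this actor's position and rotation.
; On a script message it waits a configurable delay, takes the first Ghost_girl found, transforms her and records her start location.
; A rate-adjusted timeline lerps her there by teleporting each update, with a Started flag blocking re-entry.
; On finish it messages linked actors with the player character, snaps her capsule into place and re-arms.
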(event `/Game/blueprints/scripting/base/Scripting_events.Recive_script`
  (params (player_activator :type "Character Object Reference"))
  (`KismetSystemLibrary.Delay` (`self.Delay_on_script`))
  (if (not (`self.Started`))
    (set `self.Started` true)
    (bind _outactors (`GameplayStatics.GetAllActorsOfClass` "/Game/blueprints/player_characters/ghost_girl.ghost_girl_C"))
    (bind _output_get (set `self.ghost_char` (`|GetArrayItem` _outactors)))
    (`/Game/blueprints/player_characters/ghost_girl.Transform` _output_get "NewEnumerator2")
    (`KismetSystemLibrary.Delay` 0.2)
    (set `self.char_old_location` (`SceneComponent.K2_GetComponentLocation` (`Character.CapsuleComponent` (`self.ghost_char`))))
    (`TimelineComponent.SetPlayRate` (`self.Timeline_0`) (`self.rate`))
    (`self.move`)))

(event `move`
  (bind (_direction _alpha) (`Timeline|Timeline_0` :!via `PlayFromStart`)
    (:`Update`
      (`self.K2_TeleportTo` (`self.ghost_char`) (`KismetMathLibrary.VLerp` (`self.char_old_location`) (`SceneComponent.K2_GetComponentLocation` (`self.DefaultSceneRoot`)) _alpha) (`SceneComponent.K2_GetComponentRotation` (`self.DefaultSceneRoot`))))
    (:`Finished`
      (for _array_element (`self.actors_to_activate_on_finish`)
        (message `/Game/blueprints/scripting/base/Scripting_events.Recive_script` _array_element (`GameplayStatics.GetPlayerCharacter` 0)))
      (`SceneComponent.K2_SetWorldLocationAndRotation` (`Character.CapsuleComponent` (`self.ghost_char`)) (`SceneComponent.K2_GetComponentLocation` (`self.DefaultSceneRoot`)) (`SceneComponent.K2_GetComponentRotation` (`self.DefaultSceneRoot`)) false true)
      (set `self.Started` false))))

(fn `UserConstructionScript`
  (`parent.UserConstructionScript`))
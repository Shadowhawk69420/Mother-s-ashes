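; Scripting actor that switches a player's view to itself when triggered through the ReciveScriptMulti event, optionally handing it back.
; After a start delay, it blends the activator's third_person_controller view target to this actor.
; If TransitionBackToPlayer is set, it waits an end delay and blends back to the activating player.
; SkipCamera bypasses the outgoing switch and runs only the delayed return blend.
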(event `self.ReceiveBeginPlay`
  (`parent.ReceiveBeginPlay`))

(event `self.recive_script_multi`
  (params (Player_activator :type "Character Object Reference"))
  (if (`self.Skip_camera`)
    (`KismetSystemLibrary.Delay` (`self.Delay_end`) :!label _label)
    (`PlayerController.SetViewTargetWithBlend` (cast `/Game/blueprints/game_settings/third_person_controller` (`Pawn.GetController` Player_activator) :!pure true) Player_activator (`self.Blend_end`) "VTBlend_Linear" 0.0 false)
    (else
      (`KismetSystemLibrary.Delay` (`self.delay_start`))
      (`PlayerController.SetViewTargetWithBlend` (cast `/Game/blueprints/game_settings/third_person_controller` (`Pawn.GetController` Player_activator) :!pure true) self (`self.Blend_start`) "VTBlend_Linear" 0.0 false)
      (if (`self.Transition_back_to_player`)
        (goto _label)))))

(fn `UserConstructionScript`
  (`parent.UserConstructionScript`))
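; Actor Blueprint that streams in every level named in its LevelsToStream array when play begins.
; BeginPlay enters the load chain, which loads the level at CurrentLoadedLevel as visible, with blocking on load.
; It then increments the index and calls LoadNext again until the array end, so levels load sequentially through a self-calling event rather than a loop.
; The bounds check follows each load, so the first load runs unchecked.
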(event `load_next`
  (`GameplayStatics.LoadStreamLevel` (`|GetArrayItem` (`self.levels_to_stream`) (`self.current_loaded_level`)) true true :!label _label)
  (set `self.current_loaded_level` (+ (`self.current_loaded_level`) 1))
  (if (not (>= (`self.current_loaded_level`) (`KismetArrayLibrary.Array_Length` (`self.levels_to_stream`))))
    (`self.load_next`)))

(event `self.ReceiveBeginPlay`
  (goto _label))

(fn `UserConstructionScript`)
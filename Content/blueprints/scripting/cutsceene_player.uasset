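; A scripting actor that plays a configurable level sequence as a cutscene when it receives a script event.
; On ReciveScript it waits a set delay, then creates and plays a sequence player with exposed settings for state restore, input disabling, player hiding and pause at end.
; When the sequence finishes, it sends ReciveScriptMessage with the player character to each actor in ActorsToActivate, chaining further scripted actions.
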(event `/Game/blueprints/scripting/base/Scripting_events.Recive_script`
  (params (player_activator :type "Character Object Reference"))
  (`KismetSystemLibrary.Delay` (`self.delay`))
  (bind (_outactor _returnvalue) (`LevelSequencePlayer.CreateLevelSequencePlayer` (`self.cutsceene_to_play`) (make `MovieSceneSequencePlaybackSettings` false (struct) 1.0 0.0 false (`self.Restore_state`) (`self.Disable_movement_input`) (`self.Disable_look_input`) (`self.Hide_player`) false false (`self.Pause_at_end`))))
  (`MovieSceneSequencePlayer.Play` _returnvalue)
  (add `MovieSceneSequencePlayer.OnFinished` _returnvalue (delegate `Finished_cinematic`)))

(event `Finished_cinematic`
  (for _array_element (`self.actors_to_activate`)
    (message `/Game/blueprints/scripting/base/Scripting_events.Recive_script` _array_element (`GameplayStatics.GetPlayerCharacter` 0))))

(fn `UserConstructionScript`
  (`parent.UserConstructionScript`))
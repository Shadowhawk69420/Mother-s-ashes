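; A scripting trigger volume that activates a list of actors when a Player_character overlaps its box.
; The overlap calls a Trigger event, which can optionally require that character to be player-controlled.
; It then sends ReciveScriptMessage, with the character, to each listed actor implementing the Scripting_events interface, and can destroy itself after use.
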(event `self.Box.OnComponentBeginOverlap`
  (params (OverlappedComponent :type "PrimitiveComponent Object Reference") (OtherActor :type "Actor Object Reference") (OtherComp :type "PrimitiveComponent Object Reference") (OtherBodyIndex :type Integer) (bFromSweep :type Boolean) (SweepResult :type "HitResult Structure (by ref)"))
  (`self.Trigger` OtherActor))

(event `Trigger`
  (params (Object :type "Object Object Reference"))
  (cast `/Game/blueprints/player_characters/Player_character` Object)
  (if (`self.only_player`)
    (if (`Pawn.IsPlayerControlled` (cast `/Game/blueprints/player_characters/Player_character` Object :!pure true))
      (for _array_element (`self.Actors_to_activate`) :!label _label
        (if (`KismetSystemLibrary.DoesImplementInterface` _array_element "/Game/blueprints/scripting/base/Scripting_events.Scripting_events_C")
          (message `/Game/blueprints/scripting/base/Scripting_events.Recive_script` _array_element (cast `Character` Object :!pure true))))
      (if (`self.destroy on use`)
        (`self.K2_DestroyActor`)))
    (else
      (goto _label))))

(fn `UserConstructionScript`
  (`parent.UserConstructionScript`))
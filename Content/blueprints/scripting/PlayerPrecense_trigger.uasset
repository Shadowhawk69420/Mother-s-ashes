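; Multiplayer trigger volume that fires scripted events once all players are inside it.
; On overlap, the server box-traces the volume, counts actors with player controllers against all Third_person_controller instances, then messages ActorsToActivate via the Scripting_events interface, optionally destroying itself.
; If players are missing, it sets TextVisible, whose OnRep reveals a hint text that turns toward the local camera every tick.
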(event `self.ReceiveBeginPlay`
  (`parent.ReceiveBeginPlay`)
  (`SceneComponent.SetVisibility` (`self.TextRender`) false false))

(event `CLient_look_at`
  (`SceneComponent.K2_SetWorldRotation` (`self.TextRender`) (`KismetMathLibrary.FindLookAtRotation` (`SceneComponent.K2_GetComponentLocation` (`self.TextRender`)) (`SceneComponent.K2_GetComponentLocation` (`PlayerCameraManager.TransformComponent` (`PlayerController.PlayerCameraManager` (`GameplayStatics.GetPlayerController` 0))))) false true))

(event `self.ReceiveTick`
  (params (DeltaSeconds :type "Float (single-precision)"))
  (`parent.ReceiveTick` DeltaSeconds)
  (`self.CLient_look_at`))

(event `Trigger`
  (params (Object :type "Object Object Reference"))
  (bind _box (`self.Box`))
  (bind _returnvalue (`SceneComponent.K2_GetComponentLocation` _box))
  (`KismetArrayLibrary.Array_Clear` (`self.actors_detected`))
  (set `self.Current_players` 0)
  (bind _outactors (`GameplayStatics.GetAllActorsOfClass` "/Game/blueprints/game_settings/third_person_controller.third_person_controller_C"))
  (set `self.Max_players` (`KismetArrayLibrary.Array_Length` _outactors))
  (bind (_outhits _returnvalue_2) (`KismetSystemLibrary.BoxTraceMultiForObjects` :`Start` _returnvalue :`End` (+ _returnvalue (1.0 1.0 1.0)) :`HalfSize` (* (`BoxComponent.BoxExtent` (`self.Box`)) (`SceneComponent.K2_GetComponentScale` (`self.DefaultSceneRoot`))) :`Orientation` (`SceneComponent.K2_GetComponentRotation` _box) :`ObjectTypes` (`|MakeArray` "ObjectTypeQuery3" "ObjectTypeQuery4" "ObjectTypeQuery1" "ObjectTypeQuery2" :!type "EObjectTypeQuery Enum") :`DrawDebugType` "ForDuration"))
  (if _returnvalue_2
    (for _array_element _outhits
      (bind (_bblockinghit _binitialoverlap _time _distance _location _impactpoint _normal _impactnormal _physmat _hitactor) (`GameplayStatics.BreakHitResult` _array_element))
      (if (== (`KismetArrayLibrary.Array_Find` (`self.actors_detected`) _hitactor) -1)
        (`KismetArrayLibrary.Array_AddUnique` (`self.actors_detected`) _hitactor)
        (cast `/Game/blueprints/game_settings/third_person_controller` (`Pawn.GetController` (`Actor.Instigator` _hitactor)))
        (set `self.Current_players` (+ (`self.Current_players`) 1))))
    (if (>= (`self.Current_players`) (`self.Max_players`))
      (for _array_element_2 (`self.Actors_to_activate`)
        (if (`KismetSystemLibrary.DoesImplementInterface` _array_element_2 "/Game/blueprints/scripting/base/Scripting_events.Scripting_events_C")
          (message `/Game/blueprints/scripting/base/Scripting_events.Recive_script` _array_element_2 null)))
      (if (`self.destroy on use`)
        (`self.K2_DestroyActor`))
      (else
        (`self.Visible_text`)))))

(event `self.Box.OnComponentBeginOverlap`
  (params (OverlappedComponent :type "PrimitiveComponent Object Reference") (OtherActor :type "Actor Object Reference") (OtherComp :type "PrimitiveComponent Object Reference") (OtherBodyIndex :type Integer) (bFromSweep :type Boolean) (SweepResult :type "HitResult Structure (by ref)"))
  (`/Engine/EditorBlueprintResources/ActorMacros.Switch Has Authority`
    (:`Authority`
      (`self.Trigger` OtherActor))))

(event `Visible_text`
  (set `self.text_visible` true))

(fn `OnRep_text_visible`
  (`SceneComponent.SetVisibility` (`self.TextRender`) (`self.text_visible`) false))

(fn `UserConstructionScript`
  (bind (_hint_location_location _hint_location_rotation) (`KismetMathLibrary.BreakTransform` (`self.Hint_location`)))
  (`parent.UserConstructionScript`)
  (`SceneComponent.K2_SetRelativeTransform` (`self.TextRender`) (`KismetMathLibrary.MakeTransform` _hint_location_location _hint_location_rotation) false true)
  (`SceneComponent.SetWorldScale3D` (`self.TextRender`) (1.0 1.0 1.0)))
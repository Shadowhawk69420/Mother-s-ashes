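; Question mark marker actor whose text render bobs along a timeline and turns to face the player camera.
; On BeginPlay the Float timeline lerps the text between its starting relative location and a point 20 units lower.
; Tick rotates the text toward the camera manager with a look-at rotation.
; The ReciveScript event stops the float, restores the original location and recolors the text green.
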(event `self.ReceiveBeginPlay`
  (bind _relativelocation (`SceneComponent.RelativeLocation` (`self.TextRender`)))
  (set `self.location_old` _relativelocation)
  (set `self.location_edited` (+ _relativelocation (0.0 0.0 -20.0)))
  (bind (_direction _alpha) (`Timeline|float`)
    (:`Update`
      (`SceneComponent.K2_SetRelativeLocation` (`self.TextRender`) (`KismetMathLibrary.VLerp` (`self.location_old`) (`self.location_edited`) _alpha) false true))))

(event `self.ReceiveTick`
  (params (DeltaSeconds :type "Float (single-precision)"))
  (`SceneComponent.K2_SetWorldRotation` (`self.TextRender`) (`KismetMathLibrary.FindLookAtRotation` (`SceneComponent.K2_GetComponentLocation` (`self.TextRender`)) (`self.K2_GetActorLocation` (`GameplayStatics.GetPlayerCameraManager` 0))) false false))

(event `/Game/blueprints/scripting/base/Scripting_events.Recive_script`
  (params (player_activator :type "Character Object Reference"))
  (`TimelineComponent.Stop` (`self.float`))
  (`SceneComponent.K2_SetRelativeLocation` (`self.TextRender`) (`self.location_old`) false true)
  (`TextRenderComponent.SetTextRenderColor` (`self.TextRender`) (make `Color` 0 255 0 255)))

(fn `UserConstructionScript`)
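; Scripting actor that plays animations on the activating player character when its ReciveScriptMulti event fires.
; If the player has no animation started, it waits a delay and optionally lerp-teleports them to CapsuleTransform.
; It briefly resets the character's animation variables, then starts the next AnimationSequence entry, wrapping the index after AnimIndexMax.
; The SkeletalMesh and Capsule components are destroyed on BeginPlay.
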(event `self.ReceiveBeginPlay`
  (`parent.ReceiveBeginPlay`)
  (`ActorComponent.K2_DestroyComponent` (`self.SkeletalMesh`))
  (`ActorComponent.K2_DestroyComponent` (`self.Capsule`)))

(event `self.recive_script_multi`
  (params (Player_activator :type "Character Object Reference"))
  (bind (_returnvalue_location _returnvalue_rotation) (`KismetMathLibrary.BreakTransform` (`SceneComponent.K2_GetComponentToWorld` (`self.capsule_transform`))))
  (bind _asplayer_character (cast `/Game/blueprints/player_characters/Player_character` Player_activator))
  (`/Engine/EditorBlueprintResources/StandardMacros.IsValid` _asplayer_character
    (:`Is Valid`
      (if (not (`/Game/blueprints/player_characters/Player_character.start_anim` _asplayer_character))
        (`KismetSystemLibrary.Delay` (`self.delay`))
        (if (`self.Teleport_char`)
          (`/Game/blueprints/player_characters/Player_character.Teleport_character` _asplayer_character _returnvalue_location _returnvalue_rotation 5.0 true false false)
          (`KismetSystemLibrary.Delay` 0.2))
        (set `/Game/blueprints/player_characters/Player_character.cancel` true _asplayer_character)
        (set `/Game/blueprints/player_characters/Player_character.anim_sequence` "/Game/Skeletal_meshes/Explorer/animations/Eplorer_hang_idle.Eplorer_hang_idle" _asplayer_character)
        (set `/Game/blueprints/player_characters/Player_character.loop` false _asplayer_character)
        (set `/Game/blueprints/player_characters/Player_character.end_if_not_looping` true _asplayer_character)
        (set `/Game/blueprints/player_characters/Player_character.playing_anim` false _asplayer_character)
        (set `/Game/blueprints/player_characters/Player_character.start_anim` false _asplayer_character)
        (`KismetSystemLibrary.Delay` 0.01)
        (set `/Game/blueprints/player_characters/Player_character.anim_sequence` (`|GetArrayItem` (`self.animation_sequence`) (`self.Anim_current_index`)) _asplayer_character)
        (set `/Game/blueprints/player_characters/Player_character.loop` (`self.loop`) _asplayer_character)
        (set `/Game/blueprints/player_characters/Player_character.end_if_not_looping` (`self.Teleport_char`) _asplayer_character)
        (set `/Game/blueprints/player_characters/Player_character.playing_anim` true _asplayer_character)
        (set `/Game/blueprints/player_characters/Player_character.start_anim` true _asplayer_character)
        (set `self.Anim_current_index` (+ (`self.Anim_current_index`) 1))
        (if (> (`self.Anim_current_index`) (`self.Anim_index_max`))
          (set `self.Anim_current_index` 0))))))

(fn `UserConstructionScript`
  (`parent.UserConstructionScript`))
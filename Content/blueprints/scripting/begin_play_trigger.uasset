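; A scripting trigger actor that fires on its own when the level begins, activating a set of other actors after a delay.
; BeginPlay waits for ActivationDelay, then Trigger loops over ActorsToActivate and sends ReciveScriptMessage, passing the player character, to each one implementing the Scripting_events interface.
; The trigger then destroys itself, so it fires only once.
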(event `self.ReceiveBeginPlay`
  (`parent.ReceiveBeginPlay`)
  (`KismetSystemLibrary.Delay` (`self.Activation_delay`))
  (`self.Trigger` null))

(event `Trigger`
  (params (Object :type "Object Object Reference"))
  (for _array_element (`self.Actors_to_activate`)
    (if (`KismetSystemLibrary.DoesImplementInterface` _array_element "/Game/blueprints/scripting/base/Scripting_events.Scripting_events_C")
      (message `/Game/blueprints/scripting/base/Scripting_events.Recive_script` _array_element (`GameplayStatics.GetPlayerCharacter` 0))))
  (`self.K2_DestroyActor`))

(fn `UserConstructionScript`
  (`parent.UserConstructionScript`))
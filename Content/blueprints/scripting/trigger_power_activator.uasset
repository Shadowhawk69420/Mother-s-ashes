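; Scripting actor that switches on powers for player-controlled characters.
; When its ReciveScript event fires, it waits for a delay, then searches all Player_character actors in the level.
; Each one under player control gets HasPowers set to true and then has GetCutomisationObtions called on it.
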(event `self.ReceiveBeginPlay`
  (`parent.ReceiveBeginPlay`))

(event `/Game/blueprints/scripting/base/Scripting_events.Recive_script`
  (params (player_activator :type "Character Object Reference"))
  (`KismetSystemLibrary.Delay` (`self.delay`))
  (bind _outactors (`GameplayStatics.GetAllActorsOfClass` "/Game/blueprints/player_characters/Player_character.Player_character_C"))
  (for _array_element _outactors
    (if (`Pawn.IsPlayerControlled` _array_element)
      (set `/Game/blueprints/player_characters/Player_character.Has_powers` true _array_element)
      (`/Game/blueprints/player_characters/Player_character.get_cutomisation_obtions` _array_element))))

(fn `UserConstructionScript`
  (`parent.UserConstructionScript`))
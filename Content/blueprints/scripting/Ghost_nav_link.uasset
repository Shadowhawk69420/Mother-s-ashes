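; Ghost nav link that controls how a ghost_girl agent crosses when it reaches the smart link.
; On arrival it stores the ghost's MoveLocation and sets it to the ghost itself, then branches on TransitionMethod.
; One method calls JumpServer; otherwise the ghost transforms, teleports slightly above the link destination, transforms again and resumes moving to the saved location, with short delays between steps.
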(event `self.ReceiveSmartLinkReached`
  (params (Agent :type "Actor Object Reference") (Destination :type "Vector Structure (by ref)"))
  (bind _char (`self.char`))
  (bind _asghost_girl (cast `/Game/blueprints/player_characters/ghost_girl` Agent))
  (bind _output_get (set `self.char` _asghost_girl))
  (set `self.move_loc` (`/Game/blueprints/player_characters/ghost_girl.move_location` _output_get))
  (set `/Game/blueprints/player_characters/ghost_girl.move_location` _char _char)
  (if (`|EnumEquality` (`self.transition_method`) "NewEnumerator0")
    (`/Game/blueprints/player_characters/Player_character.Jump_server` (`self.char`))
    (else
      (`/Game/blueprints/player_characters/ghost_girl.Transform` (`self.char`) "NewEnumerator2")
      (`KismetSystemLibrary.Delay` 0.5)
      (`self.K2_TeleportTo` :`self` (`self.char`) :`DestLocation` (+ Destination (0.0 0.0 30.0)))
      (`KismetSystemLibrary.Delay` 0.5)
      (`/Game/blueprints/player_characters/ghost_girl.Transform` (`self.char`) "NewEnumerator0")
      (`KismetSystemLibrary.Delay` 0.2)
      (`/Game/blueprints/player_characters/ghost_girl.Move_to_new_point` (`self.char`) (`self.move_loc`)))))

(fn `UserConstructionScript`)
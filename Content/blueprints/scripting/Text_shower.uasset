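; Scripting actor that shows a text message on the activating player's HUD when triggered.
; On ReciveScriptMulti it waits StartDelay, then gets the activator's third_person_controller and its Third_person_hud.
; It passes the configured text, color and fade delay to the HUD's CreateTextWidget, doing nothing if either cast fails.
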(event `self.recive_script_multi`
  (params (Player_activator :type "Character Object Reference"))
  (`KismetSystemLibrary.Delay` (`self.Start_delay`))
  (bind _asthird_person_controller (cast `/Game/blueprints/game_settings/third_person_controller` (`Pawn.GetController` Player_activator)))
  (bind _asthird_person_hud (cast `/Game/blueprints/game_settings/Third_person_hud` (`PlayerController.GetHUD` _asthird_person_controller)))
  (`/Game/blueprints/game_settings/Third_person_hud.create_text_widget` _asthird_person_hud (`self.text_to_show`) (`self.Text_color`) (`self.fade_delay`)))

(fn `UserConstructionScript`
  (`parent.UserConstructionScript`))
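; Scripting actor that sends a chosen pawn to a target actor using AI MoveTo.
; A ReciveScript event starts the move after a configurable delay.
; Overlapping its box component starts the same move immediately when collision activation is enabled, with no check on which actor overlaps.
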(event `/Game/blueprints/scripting/base/Scripting_events.Recive_script`
  (params (player_activator :type "Character Object Reference"))
  (`KismetSystemLibrary.Delay` (`self.Delay_on_script`))
  (`|AIMoveTo` (`self.actor_to_move`) (0.0 0.0 0.0) (`self.move_location`) 10.0 true))

(event `self.Box.OnComponentBeginOverlap`
  (params (OverlappedComponent :type "PrimitiveComponent Object Reference") (OtherActor :type "Actor Object Reference") (OtherComp :type "PrimitiveComponent Object Reference") (OtherBodyIndex :type Integer) (bFromSweep :type Boolean) (SweepResult :type "HitResult Structure (by ref)"))
  (if (`self.collision_activates?`)
    (`|AIMoveTo` (`self.actor_to_move`) (0.0 0.0 0.0) (`self.move_location`) 10.0 true)))

(fn `UserConstructionScript`
  (`parent.UserConstructionScript`))
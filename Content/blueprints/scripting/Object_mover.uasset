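; Scripting actor that moves a referenced object from its current transform toward a target transform when triggered.
; The start transform is cached on server BeginPlay and re-read on each non-looping trigger.
; ReciveScriptMulti waits a delay, applies the play rate, then toggles playing or stopping one of two timelines, chosen by the Loop flag.
; Timeline updates lerp the object's transform with teleporting, snapping to the target on finish.
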(event `self.ReceiveBeginPlay`
  (`parent.ReceiveBeginPlay`)
  (`/Engine/EditorBlueprintResources/ActorMacros.Switch Has Authority`
    (:`Authority`
      (set `self.Object_current_transform` (`self.GetTransform` (`self.Object_to_move`))))))

(event `self.recive_script_multi`
  (params (Player_activator :type "Character Object Reference"))
  (bind _object_to_move (`self.Object_to_move`))
  (bind _object_to_move_2 (`self.Object_to_move`))
  (if (not (`self.Loop`))
    (set `self.Object_current_transform` (`self.GetTransform` (`self.Object_to_move`))))
  (`KismetSystemLibrary.Delay` (`self.delay`))
  (`TimelineComponent.SetPlayRate` (`self.Timeline_0`) (`self.Play_rate`))
  (`TimelineComponent.SetPlayRate` (`self.Timeline_1`) (`self.Play_rate`))
  (if (`self.Loop`)
    (if (`self.ACTIVE`)
      (set `self.ACTIVE` false)
      (`KismetSystemLibrary.Delay` 0.2)
      (bind (_direction _alpha) (`Timeline|Timeline_1` :!via `Stop` :!label _label)
        (:`Update`
          (`self.K2_SetActorTransform` _object_to_move_2 (`KismetMathLibrary.TLerp` (`self.Object_current_transform`) (`self.Object_traquet_transform`) _alpha) false true))
        (:`Finished`
          (`self.K2_SetActorTransform` _object_to_move_2 (`self.Object_traquet_transform`) false true)))
      (else
        (set `self.ACTIVE` true)
        (`KismetSystemLibrary.Delay` 0.2)
        (goto _label)))
    (elif (`self.ACTIVE`)
      (set `self.ACTIVE` false)
      (`KismetSystemLibrary.Delay` 0.2)
      (bind (_direction_2 _alpha_2) (`Timeline|Timeline_0` :!via `Stop` :!label _label_2)
        (:`Update`
          (`self.K2_SetActorTransform` _object_to_move (`KismetMathLibrary.TLerp` (`self.Object_current_transform`) (`self.Object_traquet_transform`) _alpha_2) false true))
        (:`Finished`
          (`self.K2_SetActorTransform` _object_to_move (`self.Object_traquet_transform`) false true)))
      (else
        (set `self.ACTIVE` true)
        (`KismetSystemLibrary.Delay` 0.2)
        (goto _label_2)))))

(fn `UserConstructionScript`
  (`parent.UserConstructionScript`))
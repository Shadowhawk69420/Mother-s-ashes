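; Scripting trigger actor that sends the first Ghost_girl in the level to a configured MoveLocation.
; Its ReciveScript event waits a configurable delay, sets the ghost's transform mode, then moves it.
; Box overlap, if CollisionActivates is set, moves the ghost after delays without transforming it, as that call is disconnected.
; CollidedActor blocks repeat overlaps by the same actor until a delayed reset.
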(event `/Game/blueprints/scripting/base/Scripting_events.Recive_script`
  (params (player_activator :type "Character Object Reference"))
  (`KismetSystemLibrary.Delay` (`self.Delay_on_script`))
  (bind _outactors (`GameplayStatics.GetAllActorsOfClass` "/Game/blueprints/player_characters/ghost_girl.ghost_girl_C"))
  (bind _output (`|GetArrayItem` _outactors))
  (`/Game/blueprints/player_characters/ghost_girl.Transform` _output (`self.transform_mode_enter`))
  (`KismetSystemLibrary.Delay` 0.5)
  (`/Game/blueprints/player_characters/ghost_girl.Move_to_new_point` _output (`self.move_location`)))

(event `self.Box.OnComponentBeginOverlap`
  (params (OverlappedComponent :type "PrimitiveComponent Object Reference") (OtherActor :type "Actor Object Reference") (OtherComp :type "PrimitiveComponent Object Reference") (OtherBodyIndex :type Integer) (bFromSweep :type Boolean) (SweepResult :type "HitResult Structure (by ref)"))
  (if (not (== OtherActor (`self.collided_actor`)))
    (set `self.collided_actor` OtherActor)
    (if (`self.collision_activates?`)
      (bind _outactors (`GameplayStatics.GetAllActorsOfClass` "/Game/blueprints/player_characters/ghost_girl.ghost_girl_C"))
      (`KismetSystemLibrary.RetriggerableDelay` 1.0)
      (`KismetSystemLibrary.Delay` 0.5)
      (`/Game/blueprints/player_characters/ghost_girl.Move_to_new_point` (`|GetArrayItem` _outactors) (`self.move_location`))
      (`KismetSystemLibrary.RetriggerableDelay` 2.0)
      (set `self.collided_actor` self)
      (`KismetSystemLibrary.PrintString` "reseted"))))

(fn `UserConstructionScript`
  (`parent.UserConstructionScript`))
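; Scripting actor that plays a timed sequence of animations on a set of target skeletal mesh actors.
; ReciveScriptMulti starts the chain, which waits for the current step's delay plus short fixed delays, then plays that step's animation and loop setting on every ActorToAffect entry.
; The index advances and ReAnimate repeats the chain until it passes MaxAnimIndex, then resets to zero and stops until triggered again.
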(event `self.ReceiveBeginPlay`
  (`parent.ReceiveBeginPlay`))

(event `re_animate`
  (bind _current_anim_index (`self.Current_anim_index`))
  (`KismetSystemLibrary.Delay` (`|GetArrayItem` (`self.delay`) (`self.Current_anim_index`)) :!label _label)
  (`KismetSystemLibrary.Delay` 0.2)
  (`KismetSystemLibrary.Delay` 0.01)
  (for _array_element (`self.actor_to_affect`)
    (`SkeletalMeshComponent.PlayAnimation` (`SkeletalMeshActor.SkeletalMeshComponent` _array_element) (`|GetArrayItem` (`self.animation_sequence_1`) _current_anim_index) (`|GetArrayItem` (`self.loop`) _current_anim_index)))
  (set `self.Current_anim_index` (+ (`self.Current_anim_index`) 1))
  (if (> (`self.Current_anim_index`) (`self.Max_anim_index`))
    (set `self.Current_anim_index` 0)
    (else
      (`self.re_animate`))))

(event `self.recive_script_multi`
  (params (Player_activator :type "Character Object Reference"))
  (goto _label))

(fn `UserConstructionScript`
  (`parent.UserConstructionScript`))
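; Checkpoint trigger that sets a respawn point for the locally controlled Player_character entering its Box.
; On overlap it destroys every existing Spawn actor, then spawns a new one at the player's X/Y and rotation but the activator's own Z.
; The new Spawn's capsule world transform is written to the player's RespawnTransform, and a debug string prints the result.
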(event `self.Box.OnComponentBeginOverlap`
  (params (OverlappedComponent :type "PrimitiveComponent Object Reference") (OtherActor :type "Actor Object Reference") (OtherComp :type "PrimitiveComponent Object Reference") (OtherBodyIndex :type Integer) (bFromSweep :type Boolean) (SweepResult :type "HitResult Structure (by ref)"))
  (bind _asplayer_character (cast `/Game/blueprints/player_characters/Player_character` OtherActor :!pure true))
  (bind (_returnvalue_location _returnvalue_rotation) (`KismetMathLibrary.BreakTransform` (`self.GetTransform` _asplayer_character)))
  (if (== (`GameplayStatics.GetObjectClass` OtherActor) "/Game/blueprints/player_characters/Player_character.Player_character_C")
    (if (`Pawn.IsLocallyControlled` _asplayer_character)
      (bind _outactors (`GameplayStatics.GetAllActorsOfClass` "/Game/blueprints/scripting/Spawn.Spawn_C"))
      (for _array_element _outactors
        (`self.K2_DestroyActor` _array_element))
      (bind _output_get (set `self.Spawn_transform` (`KismetMathLibrary.MakeTransform` (`KismetMathLibrary.MakeVector` (.x _returnvalue_location) (.y _returnvalue_location) (.z (.location (`self.GetTransform`)))) _returnvalue_rotation)))
      (bind _returnvalue (`|SpawnActorFromClass` "/Game/blueprints/scripting/Spawn.Spawn_C" _output_get "AlwaysSpawn" "OverrideRootScale" null null))
      (set `self.Spawn_transform` (`SceneComponent.K2_GetComponentToWorld` (`/Game/blueprints/scripting/Spawn.Capsule` _returnvalue)))
      (bind _asplayer_character_2 (cast `/Game/blueprints/player_characters/Player_character` _asplayer_character))
      (bind _output_get_2 (set `/Game/blueprints/player_characters/Player_character.Respawn_transform` (`self.Spawn_transform`) _asplayer_character_2))
      (`KismetSystemLibrary.PrintString` (`KismetStringLibrary.Concat_StrStr` "Respawn location set : " "" (`KismetStringLibrary.Conv_TransformToString` _output_get_2)) true true (struct :`R` 0.998109 :`G` 1.0 :`A` 1.0)))))

(fn `UserConstructionScript`
  (`parent.UserConstructionScript`))
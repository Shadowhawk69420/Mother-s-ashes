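; Scripting actor that plays a set animation sequence on the player character when triggered.
; On ReciveScript it waits for a configurable delay, then finds and caches the Player_character if it is not already valid.
; It writes the sequence and non-looping, end-when-finished flags onto the character and sets its start and playing flags, leaving playback to the character.
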(event `/Game/blueprints/scripting/base/Scripting_events.Recive_script`
  (params (player_activator :type "Character Object Reference"))
  (bind _player_actor (`self.player_actor`))
  (`KismetSystemLibrary.Delay` (`self.delay`))
  (`/Engine/EditorBlueprintResources/StandardMacros.IsValid` (`self.player_actor`)
    (:`Is Valid`
      _)
    (:`Is Not Valid`
      (set `self.player_actor` (cast `/Game/blueprints/player_characters/Player_character` (`GameplayStatics.GetPlayerCharacter` 0) :!pure true))))
  (set `/Game/blueprints/player_characters/Player_character.anim_sequence` (`self.animation_to_play`) (`self.player_actor`))
  (set `/Game/blueprints/player_characters/Player_character.loop` false _player_actor)
  (set `/Game/blueprints/player_characters/Player_character.end_if_not_looping` true _player_actor)
  (set `/Game/blueprints/player_characters/Player_character.playing_anim` true _player_actor)
  (set `/Game/blueprints/player_characters/Player_character.start_anim` true _player_actor))

(fn `UserConstructionScript`
  (`parent.UserConstructionScript`))
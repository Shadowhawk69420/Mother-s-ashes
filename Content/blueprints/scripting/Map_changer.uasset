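; Map_changer is a scripted actor that ends the current map with a fade-out, then either quits to the main menu or travels to another map.
; On ReciveScriptMulti it waits a configurable delay, then plays the Fade_out level sequence with movement and look input disabled.
; When the sequence finishes, QuitToMenu selects between destroying the session to open MainMenu and issuing a Servertravel console command built from MapName.
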(event `self.ReceiveBeginPlay`
  (`parent.ReceiveBeginPlay`)
  (`/Engine/EditorBlueprintResources/ActorMacros.Switch Has Authority`))

(event `self.recive_script_multi`
  (params (Player_activator :type "Character Object Reference"))
  (`KismetSystemLibrary.Delay` (`self.delay`))
  (bind (_outactor _returnvalue) (`LevelSequencePlayer.CreateLevelSequencePlayer` "/Game/Cinematics/fade_out.fade_out" (make `MovieSceneSequencePlaybackSettings` false (struct) 1.0 0.0 false false true true false false false true)))
  (`MovieSceneSequencePlayer.Play` _returnvalue)
  (add `MovieSceneSequencePlayer.OnFinished` _returnvalue (delegate `stop`)))

(event `stop`
  (if (`self.quit_to_menu`)
    (`DestroySessionCallbackProxy.DestroySession` (`GameplayStatics.GetPlayerController` 0)
      (:`then`
        (`GameplayStatics.OpenLevel` "MainMenu")))
    (else
      (`KismetSystemLibrary.ExecuteConsoleCommand` (`KismetStringLibrary.Concat_StrStr` "Servertravel" " " (`self.Map_name`)) null))))

(fn `UserConstructionScript`
  (`parent.UserConstructionScript`))
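; Scripting actor that, when triggered, teleports the player or a chosen actor to its own location and rotation.
; ReciveScript waits a configurable delay, then moves SpecificActorToTeleport if valid, falling back to player character 0 otherwise.
; An IsNotCharacter flag moves the chosen actor by setting its transform with physics teleport and its original scale kept, instead of calling Teleport.
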(event `/Game/blueprints/scripting/base/Scripting_events.Recive_script`
  (params (player_activator :type "Character Object Reference"))
  (bind (_returnvalue_location _returnvalue_rotation) (`KismetMathLibrary.BreakTransform` (`self.GetTransform`)))
  (bind (_returnvalue_location_2 _returnvalue_rotation_2) (`KismetMathLibrary.BreakTransform` (`self.GetTransform`)))
  (bind (_returnvalue_location_3 _returnvalue_rotation_3) (`KismetMathLibrary.BreakTransform` (`self.GetTransform`)))
  (bind _specific_actor_to_teleport (`self.specific_actor_to_teleport`))
  (`KismetSystemLibrary.Delay` (`self.delay`))
  (`/Engine/EditorBlueprintResources/StandardMacros.IsValid` (`self.specific_actor_to_teleport`)
    (:`Is Valid`
      (if (`self.is_not_character`)
        (`self.K2_SetActorTransform` _specific_actor_to_teleport (`KismetMathLibrary.MakeTransform` _returnvalue_location _returnvalue_rotation (`self.GetActorScale3D` _specific_actor_to_teleport)) false true)
        (else
          (`self.K2_TeleportTo` (`self.specific_actor_to_teleport`) _returnvalue_location_3 _returnvalue_rotation_3))))
    (:`Is Not Valid`
      (`self.K2_TeleportTo` (`GameplayStatics.GetPlayerCharacter` 0) _returnvalue_location_2 _returnvalue_rotation_2))))

(fn `UserConstructionScript`
  (`parent.UserConstructionScript`))
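; Level loader Blueprint actor that streams in every level listed in its LevelsToLoad array, one after another.
; The ReciveScript event resets the index and loads the first entry with a blocking, visible-after-load LoadStreamLevel call.
; After each load it increments the index and calls LoadNext to repeat the step until the array is exhausted.
; BeginPlay, Tick and overlap events are disabled, so loading starts only when externally triggered.
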(event `load_next`
  (`GameplayStatics.LoadStreamLevel` (`|GetArrayItem` (`self.levels_to_load`) (`self.current_loaded_level`)) true true :!label _label)
  (set `self.current_loaded_level` (+ (`self.current_loaded_level`) 1))
  (if (not (>= (`self.current_loaded_level`) (`KismetArrayLibrary.Array_Length` (`self.levels_to_load`))))
    (`self.load_next`)))

(event `/Game/blueprints/scripting/base/Scripting_events.Recive_script`
  (params (player_activator :type "Character Object Reference"))
  (set `self.current_loaded_level` 0)
  (goto _label))

(fn `UserConstructionScript`
  (`parent.UserConstructionScript`))
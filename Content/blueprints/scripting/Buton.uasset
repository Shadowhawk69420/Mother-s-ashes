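; Interactable button that sends script messages to linked actors when an overlapping player interacts.
; Box overlap, gated by Enabled (settable by script), starts a looping timer replacing Tick, which checks input and shows an E-key billboard above the local player.
; With interaction animation, it fires instant targets, snaps the player into place and cycles paired player/switch animations.
; Delayed targets receive Scripting_events calls, then it locks temporarily, optionally destroying its trigger box.
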(event `interaction_anim`
  ;[1 1 1] Tick_logic
  (`self.Play_switch_an_player_anims`))

(event `start_timer`
  ;[1 1 1] Tick_logic
  (bind _returnvalue (`KismetSystemLibrary.K2_SetTimerDelegate` (delegate `Fake_tick`) 0.1 true :!label _label))
  (set `self.TImer` _returnvalue))

(event `Reset_timer`
  ;[1 1 1] Tick_logic
  (goto _label))

(event `stop_timer`
  ;[1 1 1] Tick_logic
  (`KismetSystemLibrary.K2_ClearAndInvalidateTimerHandle` (`self.TImer`)))

(event `Tick_server`
  ;[1 1 1] Tick_logic
  (if (`self.Overlapped_player_char`)
    (if (`self.locked`)
      _
      (elif (`/Game/blueprints/player_characters/Player_character.interacted` (`self.overlapped_character`))
        (if (`self.Use_interaction_anim`)
          (`|ExecutionSequence`
            (:`then_0`
              (`self.Instant_activation`))
            (:`then_1`
              (`self.interaction_anim`)
              (`/Engine/EditorBlueprintResources/StandardMacros.DoOnce` false :!label _label_2
                (:`Completed`
                  (set `self.Activate` true)
                  (`KismetSystemLibrary.Delay` 0.2)
                  (set `self.Activate` false))))
            (:`then_2`
              (`KismetSystemLibrary.Delay` (`self.Activation_delay`))
              (`/Engine/EditorBlueprintResources/StandardMacros.DoOnce` false :!label _label_3
                (:`Completed`
                  (`|ExecutionSequence`
                    (:`then_1`
                      (for _array_element (`self.actors_to_activate`)
                        (if (`KismetSystemLibrary.DoesImplementInterface` _array_element "/Game/blueprints/scripting/base/Scripting_events.Scripting_events_C")
                          (message `/Game/blueprints/scripting/base/Scripting_events.Recive_script` _array_element (`self.overlapped_character`))))
                      (if (`self.destroy_on_use`)
                        (`ActorComponent.K2_DestroyComponent` (`self.Box`))
                        (set `self.overlapped_character` null)
                        (set `self.Activate` false)
                        (else
                          (`KismetSystemLibrary.RetriggerableDelay` 0.2)
                          (`|ExecutionSequence`
                            (:`then_0`
                              (goto _label_2 :!via `Reset`))
                            (:`then_1`
                              (goto _label_3 :!via `Reset`))))))
                    (:`then_2`
                      (set `self.locked` true)
                      (`KismetSystemLibrary.RetriggerableDelay` (`self.Usage_delay`))
                      (set `self.locked` false)))))))
          (else
            (goto _label_3)))))))

(event `Fake_tick`
  ;[1 1 1] Tick_logic
  (`self.Tick_server`)
  (if (`Pawn.IsLocallyControlled` (`self.overlapped_character`))
    (if (`self.Overlapped_player_char`)
      (`self.Set_simbol_on_player`)
      (if (`self.Activate`)
        (`BillboardComponent.SetSprite` (`self.Billboard`) "/Game/textures/E_key_2.E_key_2")
        (`KismetSystemLibrary.Delay` 0.2)
        (`BillboardComponent.SetSprite` (`self.Billboard`) "/Game/textures/E_key_1.E_key_1")))))

(event `/Game/blueprints/scripting/base/Scripting_events.Recive_script`
  (params (player_activator :type "Character Object Reference"))
  ;[1 1 1] Tick_logic
  (if (not (`self.enabled`))
    (set `self.enabled` true)))

(event `self.Box.OnComponentBeginOverlap`
  (params (OverlappedComponent :type "PrimitiveComponent Object Reference") (OtherActor :type "Actor Object Reference") (OtherComp :type "PrimitiveComponent Object Reference") (OtherBodyIndex :type Integer) (bFromSweep :type Boolean) (SweepResult :type "HitResult Structure (by ref)"))
  ;[1 1 1] Detecing_collision with player
  (if (`self.enabled`)
    (cast `/Game/blueprints/player_characters/Player_character` OtherActor)
    (if (not (`self.Overlapped_player_char`))
      (set `self.overlapped_character` (cast `/Game/blueprints/player_characters/Player_character` OtherActor :!pure true))
      (set `self.Overlapped_player_char` true)
      (`self.start_timer`))))

(event `self.Box.OnComponentEndOverlap`
  (params (OverlappedComponent :type "PrimitiveComponent Object Reference") (OtherActor :type "Actor Object Reference") (OtherComp :type "PrimitiveComponent Object Reference") (OtherBodyIndex :type Integer))
  ;[1 1 1] Detecing_collision with player
  (cast `/Game/blueprints/player_characters/Player_character` OtherActor)
  (if (`self.Overlapped_player_char`)
    (set `self.Overlapped_player_char` false)
    (`self.stop_timer`)
    (`self.Set_simbol_on_player`)))

(fn `Instant_activation`
  (for _array_element (`self.actors_to_instantly_activate`)
    (if (`KismetSystemLibrary.DoesImplementInterface` _array_element "/Game/blueprints/scripting/base/Scripting_events.Scripting_events_C")
      (message `/Game/blueprints/scripting/base/Scripting_events.Recive_script` _array_element (`self.overlapped_character`)))))

(fn `Set_simbol_on_player`
  (bind _billboard (`self.Billboard`))
  (if (`self.Overlapped_player_char`)
    (`SceneComponent.SetHiddenInGame` _billboard false false)
    (`SceneComponent.K2_SetWorldLocation` (`self.Billboard`) (+ (`self.K2_GetActorLocation` (`self.overlapped_character`)) (0.0 0.0 100.0)) false true)
    (else
      (`SceneComponent.SetHiddenInGame` _billboard true false))))

(fn `UserConstructionScript`
  (`parent.UserConstructionScript`))
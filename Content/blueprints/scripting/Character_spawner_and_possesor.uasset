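; Scripting actor that replaces the player's character with a newly spawned one at its own location.
; On ReciveScript it waits a configurable delay, then spawns CharacterToSpawn at its root transform, ignoring collisions.
; The first player controller possesses the spawn, then the old character is destroyed and the new one is teleported onto the root transform.
; The preceding UnPossess targets the old character's LastHitBy controller rather than the player controller.
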(event `/Game/blueprints/scripting/base/Scripting_events.Recive_script`
  (params (player_activator :type "Character Object Reference"))
  (bind (_returnvalue_location _returnvalue_rotation) (`KismetMathLibrary.BreakTransform` (`SceneComponent.K2_GetComponentToWorld` (`self.DefaultSceneRoot`))))
  (`KismetSystemLibrary.Delay` (`self.delay`))
  (bind _output_get (set `self.old_char` (`GameplayStatics.GetPlayerCharacter` 0)))
  (`Controller.UnPossess` (`Pawn.LastHitBy` _output_get))
  (bind _returnvalue (`|SpawnActorFromClass` (`self.character_to_spawn`) (`SceneComponent.K2_GetComponentToWorld` (`self.DefaultSceneRoot`)) "AlwaysSpawn" "OverrideRootScale" null null))
  (`Controller.Possess` (`GameplayStatics.GetPlayerController` 0) _returnvalue)
  (`self.K2_DestroyActor` (`self.old_char`))
  (`self.K2_TeleportTo` _returnvalue _returnvalue_location _returnvalue_rotation))

(fn `UserConstructionScript`
  (`parent.UserConstructionScript`))
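; Ghost girl character that follows AI move targets and switches between walking, floating and spirit ball forms, also bound to keys 1–3.
; TransformFunction swaps mesh, animation, capsule, movement and collision per form, with particle effects and a pose-following opacity mesh.
; AI MoveTo success sets walking.
; Invalid or blocked moves run a line trace: despite PathIsNotBlocked's name, a hit teleports her as a ball, while a clear line floats her via timeline lerp.
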(event `self.ReceiveBeginPlay`
  (`parent.ReceiveBeginPlay`)
  (`SkinnedMeshComponent.SetLeaderPoseComponent` (`self.opacity_mesh`) (`self.SkeletalMesh`) false)
  (`KismetSystemLibrary.Delay` 1.0)
  (`self.Move_to_new_point` (`self.move_location`)))

(event `Key|One`
  (params (Key :type "Key Structure"))
  ;[1 1 1] transforming_character
  (:`Pressed`
    (`self.Transform` "NewEnumerator0")))

(event `Key|Two`
  (params (Key :type "Key Structure"))
  ;[1 1 1] transforming_character
  (:`Pressed`
    (`self.Transform` "NewEnumerator1")))

(event `Key|Three`
  (params (Key :type "Key Structure"))
  ;[1 1 1] transforming_character
  (:`Pressed`
    (`self.Transform` "NewEnumerator2")))

(event `Transform`
  (params (NewParam :type "/Game/blueprints/enums/Transform_States Enum" :default "NewEnumerator0"))
  ;[1 1 1] transforming_character
  (`self.transform_function` NewParam)
  (`SceneComponent.SetVisibility` (`self.SkeletalMesh`) true false)
  (`SceneComponent.SetVisibility` (`self.opacity_mesh`) true false))

(event `Key|U`
  (params (Key :type "Key Structure")))

(event `Move_to_new_point`
  (params (actor_to_move_to :type "Actor Object Reference"))
  (bind _returnvalue (`self.K2_GetActorLocation` (`self.move_location`)))
  (bind (_returnvalue_roll _returnvalue_pitch _returnvalue_yaw) (`KismetMathLibrary.BreakRotator` (`KismetMathLibrary.FindLookAtRotation` (`self.K2_GetActorLocation`) _returnvalue)))
  (if (!= actor_to_move_to (`self.move_location`))
    (set `self.move_location` actor_to_move_to)
    (`KismetSystemLibrary.Delay` 0.2)
    (bind _movementresult (`|AIMoveTo` self (0.0 0.0 0.0) (`self.move_location`) 5.0 true :!label _label)
      (:`then`
        (if (`|EnumEquality` _movementresult "Success")
          ;[1 1 1] walk if path is on nav mesh
          (`self.Transform` "NewEnumerator0")
          (elif (`|EnumEquality` _movementresult "Invalid")
            (`NavMovementComponent.StopMovementKeepPathing` (`self.CharacterMovement`) :!label _label_2)
            (bind _obstacle (`self.path_is_not_blocked`))
            (if _obstacle
              (`self.Transform` "NewEnumerator2")
              (`self.K2_TeleportTo` (`self.K2_GetActorLocation` (`self.move_location`)))
              (`KismetSystemLibrary.RetriggerableDelay` 1.0)
              (`self.Transform` "NewEnumerator1")
              (else
                (`self.Transform` "NewEnumerator1")
                (set `self.temp_player_location` (`SceneComponent.K2_GetComponentLocation` (`self.CapsuleComponent`)))
                (bind (_direction _aplha) (`Timeline|interp_to_new_location` :!via `PlayFromStart`)
                  (:`Update`
                    (`SceneComponent.K2_SetWorldLocation` (`self.CapsuleComponent`) (`KismetMathLibrary.VLerp` (`self.temp_player_location`) _returnvalue _aplha) false true)
                    (`self.K2_SetActorRotation` (`KismetMathLibrary.MakeRotator` 0.0 0.0 _returnvalue_yaw) true)))))
            (elif (`|EnumEquality` _movementresult "Aborted")
              (`KismetSystemLibrary.Delay` 0.2)
              (goto _label)
              (elif (`|EnumEquality` _movementresult "Blocked")
                (goto _label_2)))))))))

(fn `path_is_not_blocked`
  (returns (obstacle :type Boolean))
  (bind (_outhit _returnvalue) (`KismetSystemLibrary.LineTraceSingleForObjects` :`Start` (`SceneComponent.K2_GetComponentLocation` (`self.CapsuleComponent`)) :`End` (`self.K2_GetActorLocation` (`self.move_location`)) :`ObjectTypes` (`|MakeArray` "ObjectTypeQuery1" :!type "EObjectTypeQuery Enum") :`bTraceComplex` true :`DrawDebugType` "ForDuration"))
  (if _returnvalue
    (return true)
    (else
      (return false))))

(fn `transform_function`
  (params (Index :type "/Game/blueprints/enums/Transform_States Enum" :default "NewEnumerator0"))
  (locals (transform_option :type "/Game/blueprints/enums/Transform_States Enum" :default "NewEnumerator0"))
  (bind _returnvalue (select `/Game/blueprints/enums/Transform_States` (`local.transform_option`) :`NewEnumerator0` "MOVE_Walking" :`NewEnumerator1` "MOVE_Flying" :`NewEnumerator2` "MOVE_Flying" :!type "EMovementMode Enum"))
  (bind _output_get (set `local.transform_option` Index))
  (`SkinnedMeshComponent.SetSkinnedAssetAndUpdate` (`self.SkeletalMesh`) (select `/Game/blueprints/enums/Transform_States` _output_get :`NewEnumerator0` "/Game/Skeletal_meshes/Explorer/Ghost_girl_no_face.Ghost_girl_no_face" :`NewEnumerator1` "/Game/Skeletal_meshes/Explorer/Ghost_girl_no_face.Ghost_girl_no_face" :`NewEnumerator2` "/Game/Skeletal_meshes/spirit/Spirit_ball.Spirit_ball" :!type "SkeletalMesh Object Reference") false)
  (`SkinnedMeshComponent.SetSkinnedAssetAndUpdate` (`self.opacity_mesh`) (select `/Game/blueprints/enums/Transform_States` _output_get :`NewEnumerator0` "/Game/Skeletal_meshes/Explorer/Ghost_girl_no_face.Ghost_girl_no_face" :`NewEnumerator1` "/Game/Skeletal_meshes/Explorer/Ghost_girl_no_face.Ghost_girl_no_face" :`NewEnumerator2` "/Game/Skeletal_meshes/spirit/Spirit_ball.Spirit_ball" :!type "SkeletalMesh Object Reference") false)
  (`|ExecutionSequence`
    (:`then_0`
      (if (`|EnumInequality` (`local.transform_option`) (`self.transform_temp`))
        (`GameplayStatics.SpawnEmitterAttached` "/Game/Particles/spirit_transform.spirit_transform" (`self.CapsuleComponent`) "None" (0.0 0.0 0.0) (struct) (1.0 1.0 1.0) "SnapToTarget" false)
        (set `self.transform_temp` (`local.transform_option`))))
    (:`then_1`
      (`SkeletalMeshComponent.SetAnimationMode` (`self.SkeletalMesh`) (select `/Game/blueprints/enums/Transform_States` (`local.transform_option`) :`NewEnumerator0` "AnimationBlueprint" :`NewEnumerator1` "AnimationBlueprint" :`NewEnumerator2` "AnimationCustomMode" :!type "EAnimationMode Enum"))
      (`SkeletalMeshComponent.OverrideAnimationData` (`self.SkeletalMesh`) (select `/Game/blueprints/enums/Transform_States` (`local.transform_option`) :`NewEnumerator2` "/Game/Skeletal_meshes/spirit/Spirit_ball_Anim.Spirit_ball_Anim" :!type "AnimationAsset Object Reference") true true 0.0 1.0)
      (if (not (`|EnumEquality` (`local.transform_option`) "NewEnumerator2"))
        (`SkeletalMeshComponent.K2_SetAnimInstanceClass` (`self.SkeletalMesh`) (select `/Game/blueprints/enums/Transform_States` (`local.transform_option`) :`NewEnumerator0` "/Game/Skeletal_meshes/Explorer/animations/Explorer_anim_bp.Explorer_anim_bp_C" :`NewEnumerator1` "/Game/Skeletal_meshes/Explorer/animations/ghost/Ghost_anim_bp.Ghost_anim_bp_C" :!type "Object Class Reference")))
      (`SceneComponent.K2_SetRelativeLocation` (`self.SkeletalMesh`) (`KismetMathLibrary.MakeVector` 0.0 0.0 (select `/Game/blueprints/enums/Transform_States` (`local.transform_option`) :`NewEnumerator0` -68.878967 :`NewEnumerator1` -28.878967 :!type "Float (single-precision)")) false true)
      (set `self.Capsule_og_half_height` (select `/Game/blueprints/enums/Transform_States` (`local.transform_option`) :`NewEnumerator0` 75.0 :`NewEnumerator1` 75.0 :`NewEnumerator2` 20.0 :!type "Float (single-precision)"))
      (set `self.Capsule_og_radious` (select `/Game/blueprints/enums/Transform_States` (`local.transform_option`) :`NewEnumerator0` 25.0 :`NewEnumerator1` 25.0 :`NewEnumerator2` 20.0 :!type "Float (single-precision)"))
      (`self.Reset_capsule_size`)
      (`CharacterMovementComponent.SetMovementMode` (`self.CharacterMovement`) _returnvalue 0)
      (set `self.default_movement_mode` _returnvalue)
      (set `CharacterMovementComponent.MaxFlySpeed` (select `/Game/blueprints/enums/Transform_States` (`local.transform_option`) :`NewEnumerator0` 100.0 :`NewEnumerator1` 340.0 :`NewEnumerator2` 400.0 :!type "Float (single-precision)") (`self.CharacterMovement`))
      (set `CharacterMovementComponent.BrakingDecelerationFlying` (select `/Game/blueprints/enums/Transform_States` (`local.transform_option`) :`NewEnumerator0` 3400.0 :`NewEnumerator1` 1000.0 :`NewEnumerator2` 1000.0 :!type "Float (single-precision)") (`self.CharacterMovement`))
      (`|ExecutionSequence`
        (:`then_0`
          (`PrimitiveComponent.SetCollisionResponseToChannel` (`self.CapsuleComponent`) "ECC_WorldStatic" (select `/Game/blueprints/enums/Transform_States` (`local.transform_option`) :`NewEnumerator0` "ECR_Block" :`NewEnumerator1` "ECR_Overlap" :`NewEnumerator2` "ECR_Overlap" :!type "ECollisionResponse Enum")))
        (:`then_1`
          (if (`|EnumEquality` (`local.transform_option`) "NewEnumerator2")
            (`ActorComponent.K2_DestroyComponent` (`self.particle_trail`))
            (bind _returnvalue_2 (`GameplayStatics.SpawnEmitterAttached` "/Game/Particles/spirit_trail.spirit_trail" (`self.SkeletalMesh`) "None" (0.0 0.0 0.0) (struct) (0.6 0.6 0.6) "SnapToTarget" false))
            (set `self.particle_trail` _returnvalue_2)
            (else
              (`ActorComponent.K2_DestroyComponent` (`self.particle_trail`)))))
        (:`then_2`
          (`SceneComponent.SetWorldScale3D` (`self.SkeletalMesh`) (select `/Game/blueprints/enums/Transform_States` (`local.transform_option`) :`NewEnumerator0` (19.0 19.0 19.0) :`NewEnumerator1` (13.0 13.0 13.0) :`NewEnumerator2` (35.0 35.0 35.0) :!type "Vector Structure"))
          (`SceneComponent.SetWorldScale3D` (`self.opacity_mesh`) (select `/Game/blueprints/enums/Transform_States` (`local.transform_option`) :`NewEnumerator0` (19.0 19.0 19.0) :`NewEnumerator1` (13.0 13.0 13.0) :`NewEnumerator2` (35.0 35.0 35.0) :!type "Vector Structure"))
          (`SceneComponent.SetVisibility` (`self.SkeletalMesh`) false false)
          (`SceneComponent.SetVisibility` (`self.opacity_mesh`) false false))))))

(fn `UserConstructionScript`
  (`parent.UserConstructionScript`)
  (`SkinnedMeshComponent.SetLeaderPoseComponent` (`self.opacity_mesh`) (`self.SkeletalMesh`) true))
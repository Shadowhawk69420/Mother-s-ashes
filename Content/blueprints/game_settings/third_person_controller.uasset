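; Third-person player controller that handles dialog advancing, chat relay, pausing and saved graphics settings.
; Enter, debounced by a resetting DoOnce, advances eligible dialog boxes.
; Chat_server, on authority, calls ChatMulti on every controller to post messages to its HUD chat box; chat-focus code is unconnected.
; BeginPlay creates the settings save if missing and runs its graphics console commands, while Pause opens the HUD menu and pauses the game.
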(event `Key|Enter`
  (params (Key :type "Key Structure"))
  (:`Pressed`
    (`/Engine/EditorBlueprintResources/StandardMacros.DoOnce` false :!label _label
      (:`Completed`
        (bind _outactors (`GameplayStatics.GetAllActorsOfClass` "/Game/blueprints/scripting/DIalog_box.DIalog_box_C"))
        (for _array_element _outactors
          (if (`/Game/blueprints/scripting/DIalog_box.Can_press_enter` _array_element)
            (if (not (`/Game/blueprints/scripting/DIalog_box.in_selection` _array_element))
              (`/Game/blueprints/scripting/DIalog_box.Switch_text_line` _array_element -1))))
        (`KismetSystemLibrary.Delay` 0.1)
        (goto _label :!via `Reset`)))))

(event `Chat_server`
  (params (Box_color :type "LinearColor Structure") (Player_name :type Text) (Text_chat :type Text) (Custom_color :type Boolean) (Text_custom_color :type "SlateColor Structure"))
  (`/Engine/EditorBlueprintResources/ActorMacros.Switch Has Authority`
    (:`Authority`
      (bind _outactors (`GameplayStatics.GetAllActorsOfClass` "third_person_controller_C"))
      (for _array_element _outactors
        (`self.Chat_multi` _array_element Box_color Player_name Text_chat Custom_color Text_custom_color)))))

(event `Chat_multi`
  (params (Box_color :type "LinearColor Structure") (Player_name :type Text) (Text_chat :type Text) (Custom_color :type Boolean) (Text_custom_color :type "SlateColor Structure"))
  (bind _asthird_person_hud (cast `/Game/blueprints/game_settings/Third_person_hud` (`self.GetHUD`)))
  (bind _asgame_widget (cast `/Game/Widgets/gameplay/Game_widget` (`/Game/blueprints/game_settings/Third_person_hud.Chat_hud` _asthird_person_hud)))
  (`/Game/Widgets/gameplay/Chat_box.Chat` (`/Game/Widgets/gameplay/Game_widget.Chat_box` _asgame_widget) Box_color Player_name Text_chat Custom_color Text_custom_color))

(event `InputAction|Chat`
  (params (Key :type "Key Structure")))

(event `self.ReceiveBeginPlay`
  (bind _returnvalue (`GameplayStatics.DoesSaveGameExist` "settings"))
  (if (not _returnvalue)
    (bind _returnvalue_2 (`GameplayStatics.CreateSaveGameObject` "/Game/Settings_save.Settings_save_C"))
    (`GameplayStatics.SaveGameToSlot` _returnvalue_2 "settings"))
  (bind _returnvalue_3 (`GameplayStatics.LoadGameFromSlot` "settings"))
  (bind _assettings_save (cast `/Game/Settings_save` _returnvalue_3))
  (for _array_element (`/Game/Settings_save.Graphics_cmds` _assettings_save)
    (`KismetSystemLibrary.ExecuteConsoleCommand` _array_element null)))

(event `InputAction|Pause`
  (params (Key :type "Key Structure"))
  (:`Pressed`
    (if (not (`self.Game_paused`))
      (set `self.Game_paused` true)
      (bind _asthird_person_hud (cast `/Game/blueprints/game_settings/Third_person_hud` (`self.GetHUD`)))
      (`/Game/blueprints/game_settings/Third_person_hud.Create_pause` _asthird_person_hud)
      (set `self.bShowMouseCursor` true)
      (`GameplayStatics.SetGamePaused` true))))

(fn `UserConstructionScript`)
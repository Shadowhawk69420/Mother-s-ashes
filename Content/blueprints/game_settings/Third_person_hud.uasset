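; Third-person HUD that creates and manages the player's on-screen widgets.
; On BeginPlay, a local player controller triggers creation of the game/chat, power icon and reticle widgets.
; Events add or remove a single pause widget and replace any current fading text message with a new one.
; The dialog event creates or reuses one text box for speaker, text and replies, or animates it out on request.
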(event `Remove_pause`
  (`Widget.RemoveFromParent` (`self.Pause_widget`))
  (set `self.Pause_widget` null))

(event `Create_pause`
  (`/Engine/EditorBlueprintResources/StandardMacros.IsValid` (`self.Pause_widget`)
    (:`Is Not Valid`
      (bind _returnvalue (`|CreateWidget` "/Game/Widgets/Pause_widget.Pause_widget_C" (`self.PlayerOwner`)))
      (bind _output_get (set `self.Pause_widget` _returnvalue))
      (`UserWidget.AddToViewport` _output_get 0))))

(event `execute_client`
  (bind _returnvalue (`|CreateWidget` "/Game/Widgets/gameplay/Game_widget.Game_widget_C" (`self.PlayerOwner`)))
  (bind _output_get (set `self.Chat_hud` _returnvalue))
  (`UserWidget.AddToViewport` _output_get 0)
  (bind _returnvalue_2 (`|CreateWidget` "/Game/Widgets/gameplay/Power_icons.Power_icons_C" (`self.PlayerOwner`)))
  (bind _output_get_2 (set `self.Icon_wigets` _returnvalue_2))
  (`UserWidget.AddToViewport` _output_get_2 0)
  (bind _returnvalue_3 (`|CreateWidget` "/Game/Widgets/gameplay/Reticle_widget.Reticle_widget_C" (`self.PlayerOwner`)))
  (bind _output_get_3 (set `self.reticle_widget` _returnvalue_3))
  (`UserWidget.AddToViewport` _output_get_3 0))

(event `self.ReceiveBeginPlay`
  (if (`Controller.IsLocalPlayerController` (`self.PlayerOwner`))
    (`self.execute_client`)))

(event `create_text_widget`
  (params (Text :type Text) (color :type "LinearColor Structure" :default (struct :`R` 1.0 :`G` 1.0 :`B` 1.0 :`A` 1.0)) (fade_delay :type "Float (double-precision)"))
  (`/Engine/EditorBlueprintResources/StandardMacros.IsValid` (`self.Text_widget_var`)
    (:`Is Valid`
      (`Widget.RemoveFromParent` (`self.Text_widget_var`)))
    (:`Is Not Valid`
      _))
  (bind _returnvalue (`|CreateWidget` "/Game/Widgets/gameplay/Text_widget.Text_widget_C" (`self.PlayerOwner`) Text color fade_delay))
  (bind _output_get (set `self.Text_widget_var` _returnvalue))
  (`UserWidget.AddToViewport` _output_get 0))

(event `Create_dialog_box`
  (params (Talker_name :type Text) (Text_to_show :type Text) (show_continie_arrow :type Boolean) (Remove_box :type Boolean) (Show_replies :type Boolean) (Replies :type "Array of Text (by ref)"))
  (bind _dialog_box_wiget (`self.Dialog_box_wiget`))
  (`/Engine/EditorBlueprintResources/StandardMacros.IsValid` (`self.Dialog_box_wiget`)
    (:`Is Valid`
      (`|ExecutionSequence`
        (:`then_0`
          (if (not (not Remove_box))
            (`/Game/Widgets/gameplay/Text_box_widget.Remove_anim` (`self.Dialog_box_wiget`))
            (set `self.Dialog_box_wiget` null)))
        (:`then_1`
          (`|ExecutionSequence` :!label _label
            (:`then_0`
              (`/Game/Widgets/gameplay/Text_box_widget.Show_display_text` _dialog_box_wiget Talker_name Text_to_show show_continie_arrow Show_replies Replies))
            (:`then_1`
              (if (`KismetSystemLibrary.IsValid` (`self.Dialog_box_wiget`))
                (`UserWidget.AddToViewport` _dialog_box_wiget 0)))))))
    (:`Is Not Valid`
      (bind _returnvalue (`|CreateWidget` "/Game/Widgets/gameplay/Text_box_widget.Text_box_widget_C" (`self.PlayerOwner`)))
      (set `self.Dialog_box_wiget` _returnvalue)
      (goto _label))))

(fn `UserConstructionScript`)
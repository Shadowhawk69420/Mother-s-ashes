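; Climbable ledge actor that carries a ClimbPoint box, an optional ledge visual and a CanWalkOver flag.
; The construction script shows or hides VisualLedge according to ShowLedge, both in editor and in game.
; The event graph has no active logic.
; A disconnected box trace at ClimbPoint would clear CanWalkOver when it hits WorldStatic geometry, but it never runs.
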(event `self.ReceiveBeginPlay`)

(fn `UserConstructionScript`
  (bind _show_ledge (`self.Show_ledge`))
  (`SceneComponent.SetHiddenInGame` (`self.Visual_ledge`) (not _show_ledge) false)
  (`SceneComponent.SetVisibility` (`self.Visual_ledge`) _show_ledge false))
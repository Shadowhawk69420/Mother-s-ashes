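; Movable, climbable box pawn that the player possesses through the telekinesis power, handing control back to the owning character when that input is released.
; While possessed, mouse input rotates the view and movement follows the camera, using a helper plane kept at camera yaw for the forward direction.
; A timeline blends the mesh's glow between a default color and the flashlight color from the customisation save, which is created if missing, on possess and unpossess.
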(event `self.ReceiveBeginPlay`
  ;[1 1 1] begin_play_events an functions
  (bind _returnvalue (`GameplayStatics.DoesSaveGameExist` "customisation"))
  (if (not _returnvalue)
    (bind _returnvalue_2 (`GameplayStatics.CreateSaveGameObject` "/Game/Customisation.Customisation_C"))
    (`GameplayStatics.SaveGameToSlot` _returnvalue_2 "customisation"))
  (bind _returnvalue_3 (`GameplayStatics.LoadGameFromSlot` "customisation"))
  (bind _ascustomisation (cast `/Game/Customisation` _returnvalue_3))
  (bind (_flashlight_color_r _flashlight_color_g _flashlight_color_b) (break `LinearColor` (`/Game/Customisation.Flashlight_color` _ascustomisation)))
  (set `self.light_color_custom` (make `LinearColor` _flashlight_color_r _flashlight_color_g _flashlight_color_b 1.0))
  (`KismetSystemLibrary.Delay` 0.2)
  (`self.set_glow_color` (`self.light_color_default`)))

(event `self.ReceiveTick`
  (params (DeltaSeconds :type "Float (single-precision)"))
  (bind (_returnvalue_roll _returnvalue_pitch _returnvalue_yaw) (`KismetMathLibrary.BreakRotator` (`SceneComponent.K2_GetComponentRotation` (`self.Camera`))))
  ;[1 1 1] calculate_movment_forwards irection
  (`SceneComponent.K2_SetWorldRotation` (`self.Plane`) (`KismetMathLibrary.MakeRotator` 0.0 0.0 _returnvalue_yaw) false false))

(event `InputAction|Telequinesis`
  (params (Key :type "Key Structure"))
  (bind _owner_character (`self.owner_character`))
  ;[1 1 1] unpossing_input
  (:`Released`
    (`Controller.Possess` (`GameplayStatics.GetPlayerController` 0) _owner_character)
    (set `/Game/blueprints/player_characters/Player_character.telequinesis` false _owner_character)
    (`KismetArrayLibrary.Array_Set` (`/Game/blueprints/player_characters/Player_character.Powers_Pressed_State` _owner_character) 0 "NewEnumerator0")))

(event `InputAxis|Mouse_x`
  (params (AxisValue :type "Float (single-precision)"))
  ;[1 1 1] mouse Look
  (`self.AddControllerYawInput` AxisValue))

(event `self.ReceivePossessed`
  (params (NewController :type "Controller Object Reference"))
  ;[1 1 1] posesed and unpossesed_events
  (`self.Timeline_color_change` (`self.light_color_custom`)))

(event `InputAxis|Mouse_y`
  (params (AxisValue :type "Float (single-precision)"))
  ;[1 1 1] mouse Look
  (`self.AddControllerPitchInput` AxisValue))

(event `self.ReceiveUnpossessed`
  (params (OldController :type "Controller Object Reference"))
  ;[1 1 1] posesed and unpossesed_events
  (`self.Timeline_color_change` (`self.light_color_default`)))

(event `Timeline_color_change`
  (params (ligth_new :type "LinearColor Structure"))
  (set `self.ligth_new` ligth_new)
  (bind (_direction _alpha) (`Timeline|Timeline_0` :!via `PlayFromStart`)
    (:`Update`
      (bind _output_get (set `self.ligth_current` (`KismetMathLibrary.Conv_VectorToLinearColor` (`KismetMathLibrary.VLerp` (`KismetMathLibrary.Conv_LinearColorToVector` (`self.light_old`)) (`KismetMathLibrary.Conv_LinearColorToVector` (`self.ligth_new`)) _alpha))))
      (`self.set_glow_color` _output_get))
    (:`Finished`
      (set `self.light_old` (`self.ligth_current`)))))

(event `InputAxis|Forwards`
  (params (AxisValue :type "Float (single-precision)"))
  ;[1 1 1] movement_inputs
  (`self.AddMovementInput` (`KismetMathLibrary.Normal` (`SceneComponent.GetForwardVector` (`self.Plane`))) AxisValue))

(event `InputAxis|Strafe`
  (params (AxisValue :type "Float (single-precision)"))
  ;[1 1 1] movement_inputs
  (`self.AddMovementInput` (`SceneComponent.GetRightVector` (`self.Camera`)) AxisValue))

(fn `set_glow_color`
  (params (InLinearColor :type "LinearColor Structure"))
  (`MeshComponent.SetVectorParameterValueOnMaterials` (`self.StaticMesh`) "Glow_color" (`KismetMathLibrary.Conv_LinearColorToVector` InLinearColor)))

(fn `UserConstructionScript`)
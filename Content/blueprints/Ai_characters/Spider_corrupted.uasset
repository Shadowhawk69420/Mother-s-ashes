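; Corrupted spider enemy AI that chases the player once spotted and deals random melee damage when in range.
; On reaching the player, a sphere trace ignoring AI_base actors finds a pawn to damage and briefly raises the Attacking flag.
; A timer then rechecks range to either attack again or resume the chase while health remains.
; Death swaps to a death mesh with physics, disables movement and capsule collision, and clears that timer.
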(event `self.event_killed`
  ;[1 1 1] killed_events
  (`parent.event_killed`)
  (`SkinnedMeshComponent.SetSkinnedAssetAndUpdate` (`self.SkeletalMesh`) (`self.Death_mesh`) true)
  (`PrimitiveComponent.SetSimulatePhysics` (`self.SkeletalMesh`) true)
  (`ActorComponent.Deactivate` (`self.CharacterMovement`))
  (`PrimitiveComponent.SetCollisionEnabled` (`self.CapsuleComponent`) "NoCollision")
  (`KismetSystemLibrary.K2_ClearAndInvalidateTimerHandle` (`self.hit_reset_timer`)))

(event `Move_to_tarquet`
  (`self.set_debug_behaviour` "Moving to player" :!label _label)
  (`|AIMoveTo` self (0.0 0.0 0.0) (`self.player_ref`) 30.0 true
    (:`OnSuccess`
      (`self.set_debug_behaviour` "attacking the player")
      (bind (_outhit _returnvalue) (`self.sphere_trace_for_player` "ForOneFrame" :!label _label_2))
      (if _returnvalue
        (message `/Game/blueprints/interfaces/Damage.Normal_damage` (`.HitActor` (`GameplayStatics.BreakHitResult` _outhit)) (`KismetMathLibrary.RandomIntegerInRange` (`self.damage_min`) (`self.damage_max`)))
        (else
          (`self.set_debug_behaviour` "Too far to hit player")))
      (set `self.Attacking` true)
      (bind _returnvalue_2 (`KismetSystemLibrary.K2_SetTimerDelegate` (delegate `Start_moving_to_player`) 2.8))
      (set `self.hit_reset_timer` _returnvalue_2)
      (`KismetSystemLibrary.Delay` 0.2)
      (set `self.Attacking` false))))

(event `Keep_hitting`
  (goto _label_2))

(event `self.Spoted player`
  (`parent.Spoted player`)
  (goto _label))

(event `Start_moving_to_player`
  (if (>= (`self.Health`) 1)
    (`self.set_debug_behaviour` "Am I close to player?")
    (bind (_outhit _returnvalue) (`self.sphere_trace_for_player` "None"))
    (if _returnvalue
      (`self.Keep_hitting`)
      (`self.set_debug_behaviour` "Re-attacking the player")
      (else
        (`self.Move_to_tarquet`)
        (`self.set_debug_behaviour` "Moving to player")))))

(fn `UserConstructionScript`
  (`parent.UserConstructionScript`))
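; Main menu ship actor that displays the customised Explorer character alongside an animated player ship.
; BeginPlay creates dynamic materials for face, body, hair and gear, then applies colours from the "customisation" save, creating it if missing; glow depends on HasPowers.
; Tick polls AnimToPlay to switch the Explorer's animation and uses Land to choose the ship's landing or hover-idle animation, each behind a never-reset DoOnce.
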(event `Update_customisation`
  (bind _explorer_body (`self.Explorer_body`))
  (bind _returnvalue (`GameplayStatics.DoesSaveGameExist` "customisation"))
  (if (not _returnvalue)
    (bind _returnvalue_2 (`GameplayStatics.CreateSaveGameObject` "/Game/Customisation.Customisation_C"))
    (`GameplayStatics.SaveGameToSlot` _returnvalue_2 "customisation"))
  (bind _returnvalue_3 (`GameplayStatics.LoadGameFromSlot` "customisation"))
  (bind _ascustomisation (cast `/Game/Customisation` _returnvalue_3))
  (set `self.Primary_color` (`/Game/Customisation.Primary_color` _ascustomisation))
  (set `self.Secondary_color` (`/Game/Customisation.Shoe_color` _ascustomisation))
  (set `self.Hair_color` (`/Game/Customisation.Hair_color` _ascustomisation))
  (set `self.Top_color` (`/Game/Customisation.Top_color` _ascustomisation))
  (set `self.Backpack_color` (`/Game/Customisation.Backpack_color` _ascustomisation))
  (set `self.flashlight` (`/Game/Customisation.Flashlight_color` _ascustomisation))
  (`|ExecutionSequence`
    (:`then_0`
      (if (`self.Has_powers`)
        (`MaterialInstanceDynamic.SetVectorParameterValue` _explorer_body "Glow_color" (`self.flashlight`))
        (`MaterialInstanceDynamic.SetVectorParameterValue` (`self.Explorer_face`) "Glow_color" (`self.flashlight`))
        (else
          (`MaterialInstanceDynamic.SetVectorParameterValue` :`self` _explorer_body :`ParameterName` "Glow_color")
          (`MaterialInstanceDynamic.SetVectorParameterValue` :`self` (`self.Explorer_face`) :`ParameterName` "Glow_color"))))
    (:`then_1`
      (`MaterialInstanceDynamic.SetVectorParameterValue` (`self.Explorer_body`) "Primary_color" (`self.Primary_color`))
      (`MaterialInstanceDynamic.SetVectorParameterValue` (`self.Explorer_gear`) "Primary_color" (`self.Primary_color`))
      (`MaterialInstanceDynamic.SetVectorParameterValue` (`self.Explorer_body`) "Secondary_color" (`self.Secondary_color`))
      (`MaterialInstanceDynamic.SetVectorParameterValue` (`self.Hair_material`) "Primary_color" (`self.Hair_color`))
      (`MaterialInstanceDynamic.SetVectorParameterValue` (`self.Explorer_body`) "Tetiary_color" (`self.Top_color`))
      (`MaterialInstanceDynamic.SetVectorParameterValue` (`self.Explorer_gear`) "Primary_color" (`self.Backpack_color`)))))

(event `self.ReceiveBeginPlay`
  (bind _returnvalue (`PrimitiveComponent.CreateDynamicMaterialInstance` (`self.explorer`) 1 "/Game/Materials/Explorer_face.Explorer_face" "None"))
  (set `self.Explorer_face` _returnvalue)
  (bind _returnvalue_2 (`PrimitiveComponent.CreateDynamicMaterialInstance` (`self.explorer`) 0 "/Game/Materials/Explorer_body_surface.Explorer_body_surface" "None"))
  (set `self.Explorer_body` _returnvalue_2)
  (bind _returnvalue_3 (`PrimitiveComponent.CreateDynamicMaterialInstance` (`self.explorer`) 2 "/Game/Materials/Explorer_hair.Explorer_hair" "None"))
  (set `self.Hair_material` _returnvalue_3)
  (bind _returnvalue_4 (`PrimitiveComponent.CreateDynamicMaterialInstance` (`self.explorer`) 6 "/Game/Materials/Explorer_gear.Explorer_gear" "None"))
  (set `self.Explorer_gear` _returnvalue_4)
  (`self.Update_customisation`))

(event `self.ReceiveTick`
  (params (DeltaSeconds :type "Float (single-precision)"))
  (bind _anim_to_play (`self.Anim_to_play`))
  (bind _skeletalmesh (`self.SkeletalMesh`))
  (bind _skeletalmesh_2 (`self.SkeletalMesh`))
  (bind _explorer (`self.explorer`))
  (`|ExecutionSequence`
    (:`then_0`
      (if (!= (`self.Anim_to_play`) (`self.Anim_to_play_old`))
        (`/Engine/EditorBlueprintResources/StandardMacros.DoOnce` false :!label _label
          (:`Completed`
            (`SkeletalMeshComponent.SetAnimationMode` (`self.explorer`) "AnimationSingleNode")
            (`SkeletalMeshComponent.SetAnimation` _explorer _anim_to_play)
            (`SkeletalMeshComponent.PlayAnimation` _explorer _anim_to_play (`self.Loop_animation`))
            (set `self.Anim_to_play_old` (`self.Anim_to_play`))
            (`KismetSystemLibrary.PrintString` "played_anim")))
        (else
          (goto _label :!via `Reset`))))
    (:`then_1`
      (if (`self.land`)
        (`/Engine/EditorBlueprintResources/StandardMacros.DoOnce` false
          (:`Completed`
            (`SkeletalMeshComponent.SetAnimationMode` (`self.SkeletalMesh`) "AnimationSingleNode")
            (`SkeletalMeshComponent.SetAnimation` _skeletalmesh "/Game/Skeletal_meshes/player_ship/player_ship_anims/Player_ship_Land.Player_ship_Land")
            (`SkeletalMeshComponent.PlayAnimation` _skeletalmesh "/Game/Skeletal_meshes/player_ship/player_ship_anims/Player_ship_Land.Player_ship_Land" (`self.Loop_animation`))))
        (else
          (`/Engine/EditorBlueprintResources/StandardMacros.DoOnce` false
            (:`Completed`
              (`SkeletalMeshComponent.SetAnimationMode` (`self.SkeletalMesh`) "AnimationSingleNode")
              (`SkeletalMeshComponent.SetAnimation` _skeletalmesh_2 "/Game/Skeletal_meshes/player_ship/player_ship_anims/Player_ship_hover_idle.Player_ship_hover_idle")
              (`SkeletalMeshComponent.PlayAnimation` _skeletalmesh_2 "/Game/Skeletal_meshes/player_ship/player_ship_anims/Player_ship_hover_idle.Player_ship_hover_idle" (`self.Loop_animation`)))))))))

(fn `UserConstructionScript`)